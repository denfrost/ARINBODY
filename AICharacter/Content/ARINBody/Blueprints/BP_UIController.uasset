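; BP_UIController is an actor that acts as a name-based command hub for the ARINBody UI panels.
; On BeginPlay it caches the CLM_LayoutWidget, whose WidgetArray FindWidget searches by name, printing each name checked.
; Wrapper functions open, close or change text on the found widget, or cast it to image, video, browser or chart panels for type-specific commands.
; ShowCharacter and HideCharacter toggle CH_ARINBody actors by teleporting them between two fixed locations.
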(event `self.ReceiveBeginPlay`
  (bind _foundwidgets (`WidgetBlueprintLibrary.GetAllWidgetsOfClass` "/Game/ARINBody/Blueprints/UI/CLM_LayoutWidget.CLM_LayoutWidget_C" false))
  (for _array_element _foundwidgets
    (set `self.LayoutWidgetRef` _array_element)))

(fn `ChangeChart`
  (params (WidgetName :type String) (ChartData :type String))
  (bind _widgetref (`self.FindWidget` WidgetName))
  (bind _asclm_chart_panel (cast `/Game/ARINBody/Blueprints/UI/CLM_ChartPanel` _widgetref))
  (`/Game/ARINBody/Blueprints/UI/CLM_ChartPanel.ChangeChart` _asclm_chart_panel ChartData))

(fn `ChangeImage`
  (params (WidgetName :type String) (ImageName :type String) (EffectStyle :type String))
  (bind _widgetref (`self.FindWidget` WidgetName))
  (bind _asclm_image_panel (cast `/Game/ARINBody/Blueprints/UI/CLM_ImagePanel` _widgetref))
  (`/Game/ARINBody/Blueprints/UI/CLM_ImagePanel.ChangeImage` _asclm_image_panel ImageName EffectStyle))

(fn `ChangeText`
  (params (WidgetName :type String) (InputText :type String) (EffectStyle :type String))
  (bind _widgetref (`self.FindWidget` WidgetName))
  (`/Game/ARINBody/Blueprints/UI/CLM_Widget.ChangeText` _widgetref InputText EffectStyle))

(fn `ChangeURL`
  (params (WidgetName :type String) (URL :type String))
  (bind _widgetref (`self.FindWidget` WidgetName))
  (bind _asclm_browser_panel (cast `/Game/ARINBody/Blueprints/UI/CLM_BrowserPanel` _widgetref))
  (`/Game/ARINBody/Blueprints/UI/CLM_BrowserPanel.ChangeURL` _asclm_browser_panel URL))

(fn `Close`
  (params (WidgetName :type String) (EffectStyle :type String))
  (bind _widgetref (`self.FindWidget` WidgetName))
  (`/Game/ARINBody/Blueprints/UI/CLM_Widget.Close` _widgetref EffectStyle))

(fn `FindWidget`
  (params (WidgetName :type String))
  (returns (WidgetRef :type "/Game/ARINBody/Blueprints/UI/CLM_Widget Object Reference"))
  (locals (Widget :type "/Game/ARINBody/Blueprints/UI/CLM_Widget Object Reference"))
  (for _array_element (`/Game/ARINBody/Blueprints/UI/CLM_LayoutWidget.WidgetArray` (`self.LayoutWidgetRef`))
    (bind _widgetname (`/Game/ARINBody/Blueprints/UI/CLM_Widget.WidgetName` _array_element))
    (`KismetSystemLibrary.PrintString` _widgetname)
    (if (`KismetStringLibrary.EqualEqual_StrStr` WidgetName _widgetname)
      (set `local.Widget` _array_element)
      (break)))
  (return (`local.Widget`)))

(fn `HideCharacter`
  (bind _outactors (`GameplayStatics.GetAllActorsOfClass` "/Game/ARINBody/Blueprints/CH_ARINBody.CH_ARINBody_C"))
  (for _array_element _outactors
    (`self.K2_SetActorLocationAndRotation` :`self` _array_element :`NewLocation` (-500.0 0.0 110.0))))

(fn `Open`
  (params (WidgetName :type String) (EffectStyle :type String))
  (bind _widgetref (`self.FindWidget` WidgetName))
  (`/Game/ARINBody/Blueprints/UI/CLM_Widget.Open` _widgetref EffectStyle))

(fn `PauseVideo`
  (params (WidgetName :type String))
  (bind _widgetref (`self.FindWidget` WidgetName))
  (bind _asclm_video_panel (cast `/Game/ARINBody/Blueprints/UI/CLM_VideoPanel` _widgetref))
  (`/Game/ARINBody/Blueprints/UI/CLM_VideoPanel.PauseVideo` _asclm_video_panel))

(fn `PlayVideo`
  (params (WidgetName :type String) (VideoPath :type String))
  (bind _widgetref (`self.FindWidget` WidgetName))
  (bind _asclm_video_panel (cast `/Game/ARINBody/Blueprints/UI/CLM_VideoPanel` _widgetref))
  (`/Game/ARINBody/Blueprints/UI/CLM_VideoPanel.PlayVideo` _asclm_video_panel VideoPath))

(fn `ShowCharacter`
  (bind _outactors (`GameplayStatics.GetAllActorsOfClass` "/Game/ARINBody/Blueprints/CH_ARINBody.CH_ARINBody_C"))
  (for _array_element _outactors
    (`self.K2_SetActorLocationAndRotation` :`self` _array_element :`NewLocation` (0.0 0.0 110.0))))

(fn `StopVideo`
  (params (WidgetName :type String))
  (bind _widgetref (`self.FindWidget` WidgetName))
  (bind _asclm_video_panel (cast `/Game/ARINBody/Blueprints/UI/CLM_VideoPanel` _widgetref))
  (`/Game/ARINBody/Blueprints/UI/CLM_VideoPanel.StopVideo` _asclm_video_panel))

(fn `UserConstructionScript`)