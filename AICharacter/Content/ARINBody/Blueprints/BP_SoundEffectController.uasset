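; BP_SoundEffectController plays, pauses and stops sound effects by name through a single Audio component.
; ImportData loads WAV files at runtime from a configurable directory into SoundList, keyed by file name without extension.
; Play looks up that map, or resumes the current sound if the same name is requested while paused.
; ShowData prints the loaded entries for debugging; the older database query in ImportData is disconnected.
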(event `self.ReceiveBeginPlay`)

(event `Key|T`
  (params (Key :type "Key Structure")))

(fn `ImportData`
  (`BlueprintMapLibrary.Map_Clear` (`self.SoundList`))
  (bind (_count _files _filepaths) (`RealTimeImportBPLibrary.LoadAllFilesFromDirectory` "E_ad" "E_wav" (`self.PathSoundEffectData`)))
  (bind _output_get (set `self.WavFileList` _files))
  (set `self.WavPathFileList` _filepaths)
  (for (_array_element _array_index) _output_get
    (bind _sound (`RealTimeImportBPLibrary.LoadWavFile` (`RealTimeImportBPLibrary.getRealTimeImportTarget`) "E_ad" (`|GetArrayItem` (`self.WavPathFileList`) _array_index) 0.0))
    (`BlueprintMapLibrary.Map_Add` (`self.SoundList`) (`|GetArrayItem` (`KismetStringLibrary.ParseIntoArray` _array_element ".")) _sound)))

(fn `InitDataPath`
  (params (PathSoundEffect :type String))
  (set `self.PathSoundEffectData` PathSoundEffect))

(fn `InitSoundDB`
  (params (DBManagerRef :type "/Game/ARINBody/Blueprints/BP_JsonDBManager Object Reference"))
  (set `self.DBManagerRef` DBManagerRef))

(fn `Pause`
  (`AudioComponent.SetPaused` (`self.Audio`) true))

(fn `Play`
  (params (FileName :type String))
  (bind _audio (`self.Audio`))
  (if (and (`self.IsPaused`) (`KismetStringLibrary.EqualEqual_StrStr` (`self.PlayingSound`) FileName))
    (`AudioComponent.SetPaused` (`self.Audio`) false)
    (else
      (`AudioComponent.SetSound` _audio (`BlueprintMapLibrary.Map_Find` (`self.SoundList`) FileName))
      (`AudioComponent.Play` _audio 0.0)
      (set `self.PlayingSound` FileName))))

(fn `ShowData`
  (`|ExecutionSequence`
    (:`then_1`
      (`KismetSystemLibrary.PrintString` (`KismetStringLibrary.Concat_StrStr` "number of sound effect  data: " (`KismetStringLibrary.Conv_IntToString` (`BlueprintMapLibrary.Map_Length` (`self.SoundList`)))) true true (struct :`R` 1.0 :`G` 0.889065 :`A` 1.0) 10.0))
    (:`then_2`
      (bind _keys (`BlueprintMapLibrary.Map_Keys` (`self.SoundList`)))
      (for (_array_element _array_index) _keys
        (`KismetSystemLibrary.PrintString` _array_element)))))

(fn `Stop`
  (`AudioComponent.Stop` (`self.Audio`)))

(fn `UserConstructionScript`)