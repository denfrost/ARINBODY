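; Lip-sync controller actor that plays speech audio and animates viseme morph targets on the player character's mesh.
; Init functions build speech sound and JSON speech-mark maps keyed by name, from project content on Android or runtime-loaded files elsewhere.
; SetVisemeMap fills the timed viseme list for a speech ID.
; Audio playback percent becomes milliseconds that step through that list, with the VisemeMap table's AmazonPolly row mapping visemes to morph targets.
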(event `self.ReceiveBeginPlay`)

(event `self.ReceiveTick`
  (params (DeltaSeconds :type "Float (single-precision)"))
  (bind _audio (`self.Audio`))
  (if (`self.IsPlaying`)
    (set `self.IsPlaying` false)
    (set `self.time` 0)
    (set `self.IsFinished` false)
    (if (not (`AudioComponent.IsPlaying` _audio))
      (`AudioComponent.Play` _audio 0.0))
    (else
      (`|ExecutionSequence`
        (:`then_0`
          (`AudioComponent.SetPaused` (`self.Audio`) (`self.bPause`)))
        (:`then_1`
          (if (`self.bStop`)
            (`AudioComponent.Stop` (`self.Audio`))))))))

(event `self.Audio.OnAudioPlaybackPercent`
  (params (PlayingSoundWave :type "SoundWave Object Reference") (PlaybackPercent :type "Float (single-precision)"))
  (bind _visemelist (`self.VisemeList`))
  (bind _mesh (`Character.Mesh` (`GameplayStatics.GetPlayerCharacter` 0)))
  (bind (_time _type _value) (break `/Game/ARINBody/Data/VisemeListStruct` (`|GetArrayItem` _visemelist (`self.VisemeIndex`))))
  (bind _output_get (set `self.time` (`KismetMathLibrary.FFloor` (* (`SoundBase.Duration` PlayingSoundWave) PlaybackPercent 1000.0))))
  (`LowEntryJsonDebugLibrary.PrintInteger` _output_get "Audio Time : " 0.0 true true (struct :`R` 1.0 :`B` 0.014804 :`A` 1.0))
  ;[1 1 1] Select Viseme Label based on speech sound time
  (if (> (- (`KismetArrayLibrary.Array_Length` _visemelist) 1) (`self.VisemeIndex`))
    (if (>= (`self.time`) _time)
      (`/Engine/EditorBlueprintResources/StandardMacros.IncrementInt` (`self.VisemeIndex`)
        (:`  `
          _)))
    (bind _output_get_2 (set `self.VisemeValue` _value))
    ;[1 1 1] Viseme Blendshape Animation
    (bind _returnvalue (`|GetDataTableRow` "/Game/ARINBody/Data/VisemeMap.VisemeMap" "AmazonPolly")
      (:`then`
        (bind _visememap (break `/Game/ARINBody/Data/VisemeMapStruct` _returnvalue))
        (bind _keys (`BlueprintMapLibrary.Map_Keys` _visememap))
        (for _array_element _keys
          (if (`KismetStringLibrary.EqualEqual_StrStr` _array_element (`self.VisemeValue`))
            (`SkeletalMeshComponent.SetMorphTarget` _mesh (`KismetStringLibrary.Conv_StringToName` (`BlueprintMapLibrary.Map_Find` _visememap _output_get_2)) 0.5 true)
            (else
              (`SkeletalMeshComponent.SetMorphTarget` _mesh (`KismetStringLibrary.Conv_StringToName` (`BlueprintMapLibrary.Map_Find` _visememap _array_element)) 0.0 true))))))))

(event `self.Audio.OnAudioFinished`
  (set `self.time` 0)
  (set `self.IsFinished` true)
  (if (`AudioComponent.IsPlaying` (`self.Audio`))
    (`AudioComponent.Stop` (`self.Audio`))))

(fn `changeSpeechSound`
  (params (SpeechList :type "Map of String to SoundBase Object Reference") (key :type String))
  (bind _value (`BlueprintMapLibrary.Map_Find` SpeechList key))
  (bind _audio (`self.Audio`))
  (`AudioComponent.SetSound` _audio _value)
  (set `AudioComponent.Sound` _value _audio))

(fn `getDurationOfSpeech`
  (params (speech_id :type String))
  (returns (duration :type "Float (double-precision)"))
  (return (`BlueprintMapLibrary.Map_Find` (`self.SpeechDurationList`) speech_id)))

(fn `InitDataPath`
  (params (PathSpeechWav :type String) (PathSpeechMarks :type String))
  (set `self.PathSpeechData` PathSpeechWav)
  (set `self.PathSpeechMarks` PathSpeechMarks))

(fn `InitLipSyncController`
  ;[1 1 1] deactivate audio start
  (`ActorComponent.Deactivate` (`self.Audio`))
  ;[1 1 1] load wav data
  (`self.InitSpeechList`)
  ;[1 1 1] load marks data into datatable
  (`self.InitVisemeMap`)
  (`self.setSpeechDurationList`))

(fn `InitSpeechList`
  (if (`LowEntryExtendedStandardLibrary.AndroidPlatform`)
    (`BlueprintMapLibrary.Map_Clear` (`self.SpeechList`))
    (for _array_element (`AssetRegistry.GetAssetsByPath` (`AssetRegistryHelpers.GetAssetRegistry`) "/Game/ARINBody/Data/Speech/SpeechWav" false false)
      (bind _assound_base (cast `SoundBase` (`AssetRegistryHelpers.GetAsset` _array_element)))
      (`BlueprintMapLibrary.Map_Add` (`self.SpeechList`) (`KismetStringLibrary.Conv_NameToString` (`.AssetName` (break `AssetData` _array_element))) _assound_base))
    (else
      (`BlueprintMapLibrary.Map_Clear` (`self.SpeechList`))
      (bind (_count _files _filepaths) (`RealTimeImportBPLibrary.LoadAllFilesFromDirectory` "E_ad" "E_wav" (`self.PathSpeechData`)))
      (bind _output_get (set `self.WavFileList` _files))
      (set `self.WavPathFileList` _filepaths)
      (for (_array_element_2 _array_index) _output_get
        (bind _sound (`RealTimeImportBPLibrary.LoadWavFile` (`RealTimeImportBPLibrary.getRealTimeImportTarget`) "E_ad" (`|GetArrayItem` (`self.WavPathFileList`) _array_index) 0.0))
        (`BlueprintMapLibrary.Map_Add` (`self.SpeechList`) (`|GetArrayItem` (`KismetStringLibrary.ParseIntoArray` _array_element_2 ".")) _sound)))))

(fn `InitVisemeMap`
  (if (`LowEntryExtendedStandardLibrary.AndroidPlatform`)
    (bind _keys (`BlueprintMapLibrary.Map_Keys` (`self.SpeechList`)))
    (for _array_element _keys
      (for _array_element_2 (`KismetStringLibrary.ParseIntoArray` (`CoreUtilityBPLibrary.Conv_BytesToString` (`LowEntryFileManagerLibrary.GetFileData` (`KismetStringLibrary.Concat_StrStr` (`KismetSystemLibrary.GetProjectContentDirectory`) "ARINBody/Data/Speech/SpeechMarks/" (`KismetStringLibrary.Concat_StrStr` _array_element ".marks")))) (`LowEntryExtendedStandardLibrary.NewlineCharacter`))
        (bind _returnjsonobjectvalue (`LowEntryJsonLibrary.Json_ParseJsonString` _array_element_2)
          (:`FoundObject`
            (bind _returnvalue (`LowEntryJsonLibrary.Object_GetString` _returnjsonobjectvalue "type")
              (:`Success`
                (switch `string` _returnvalue
                  (:`sentence`
                    (`KismetArrayLibrary.Array_Add` (`self.SentenceJSONList`) _returnjsonobjectvalue))
                  (:`word`
                    (`KismetArrayLibrary.Array_Add` (`self.WordJSONList`) _returnjsonobjectvalue))
                  (:`viseme`
                    (`KismetArrayLibrary.Array_Add` (`self.VisemeJSONList`) _returnjsonobjectvalue))))))))
      (`|ExecutionSequence`
        (:`then_0`
          (bind _jsonobject (`|LowEntry_CreateJsonObjectPure` (`LowEntryJsonLibrary.ObjectEntry_Pure_CreateFromJsonArray` "SentenceList" (`LowEntryJsonLibrary.Array_Pure_CreateFromJsonObjectArray` (`self.SentenceJSONList`))) (`LowEntryJsonLibrary.ObjectEntry_Pure_CreateFromJsonArray` "WordList" (`LowEntryJsonLibrary.Array_Pure_CreateFromJsonObjectArray` (`self.WordJSONList`))) (`LowEntryJsonLibrary.ObjectEntry_Pure_CreateFromJsonArray` "VisemeList" (`LowEntryJsonLibrary.Array_Pure_CreateFromJsonObjectArray` (`self.VisemeJSONList`))) (`LowEntryJsonLibrary.ObjectEntry_Pure_CreateFromString` "name" _array_element)))
          (`KismetArrayLibrary.Array_Add` (`self.SpeechMarksList`) _jsonobject)
          (`BlueprintMapLibrary.Map_Add` (`self.SpeechSyncList`) _array_element _jsonobject))
        (:`then_1`
          (`KismetArrayLibrary.Array_Clear` (`self.SentenceJSONList`))
          (`KismetArrayLibrary.Array_Clear` (`self.WordJSONList`))
          (`KismetArrayLibrary.Array_Clear` (`self.VisemeJSONList`)))))
    (else
      (bind (_count _files _filepaths) (`RealTimeImportBPLibrary.LoadAllFilesFromDirectory` "E_ad" "E_all" (`self.PathSpeechMarks`)))
      (bind _output_get (set `self.MarksFileList` _files))
      (bind _output_get_2 (set `self.MarksPathFileList` _filepaths))
      (for (_array_element_3 _array_index) _output_get_2
        (bind (_filename _bytes) (`RealTimeImportBPLibrary.LoadFile` "E_ad" _array_element_3))
        (for _array_element_4 (`KismetStringLibrary.ParseIntoArray` (`CoreUtilityBPLibrary.Conv_BytesToString` _bytes) (`LowEntryExtendedStandardLibrary.NewlineCharacter`))
          (bind _returnjsonobjectvalue_2 (`LowEntryJsonLibrary.Json_ParseJsonString` _array_element_4)
            (:`FoundObject`
              (bind _returnvalue_2 (`LowEntryJsonLibrary.Object_GetString` _returnjsonobjectvalue_2 "type")
                (:`Success`
                  (switch `string` _returnvalue_2
                    (:`sentence`
                      (`KismetArrayLibrary.Array_Add` (`self.SentenceJSONList`) _returnjsonobjectvalue_2))
                    (:`word`
                      (`KismetArrayLibrary.Array_Add` (`self.WordJSONList`) _returnjsonobjectvalue_2))
                    (:`viseme`
                      (`KismetArrayLibrary.Array_Add` (`self.VisemeJSONList`) _returnjsonobjectvalue_2))))))))
        (`|ExecutionSequence`
          (:`then_0`
            (bind _output (`|GetArrayItem` (`KismetStringLibrary.ParseIntoArray` (`|GetArrayItem` _output_get _array_index) ".")))
            (bind _jsonobject_2 (`|LowEntry_CreateJsonObjectPure` (`LowEntryJsonLibrary.ObjectEntry_Pure_CreateFromJsonArray` "SentenceList" (`LowEntryJsonLibrary.Array_Pure_CreateFromJsonObjectArray` (`self.SentenceJSONList`))) (`LowEntryJsonLibrary.ObjectEntry_Pure_CreateFromJsonArray` "WordList" (`LowEntryJsonLibrary.Array_Pure_CreateFromJsonObjectArray` (`self.WordJSONList`))) (`LowEntryJsonLibrary.ObjectEntry_Pure_CreateFromJsonArray` "VisemeList" (`LowEntryJsonLibrary.Array_Pure_CreateFromJsonObjectArray` (`self.VisemeJSONList`))) (`LowEntryJsonLibrary.ObjectEntry_Pure_CreateFromString` "name" _output)))
            (`KismetArrayLibrary.Array_Add` (`self.SpeechMarksList`) _jsonobject_2)
            (`BlueprintMapLibrary.Map_Add` (`self.SpeechSyncList`) _output _jsonobject_2))
          (:`then_1`
            (`KismetArrayLibrary.Array_Clear` (`self.SentenceJSONList`))
            (`KismetArrayLibrary.Array_Clear` (`self.WordJSONList`))
            (`KismetArrayLibrary.Array_Clear` (`self.VisemeJSONList`))))))))

(fn `ResetVisemeAnimation`
  (bind _mesh (`Character.Mesh` (`GameplayStatics.GetPlayerCharacter` 0)))
  (`KismetArrayLibrary.Array_Clear` (`self.VisemeList`))
  (bind _returnvalue (`|GetDataTableRow` "/Game/ARINBody/Data/VisemeMap.VisemeMap" "AmazonPolly")
    (:`then`
      (bind _visememap (break `/Game/ARINBody/Data/VisemeMapStruct` _returnvalue))
      (bind _keys (`BlueprintMapLibrary.Map_Keys` _visememap))
      (for _array_element _keys
        (if (`KismetStringLibrary.EqualEqual_StrStr` _array_element "Neutral")
          (bind _returnvalue_2 (`KismetStringLibrary.Conv_StringToName` (`BlueprintMapLibrary.Map_Find` _visememap _array_element)))
          (`SkeletalMeshComponent.SetMorphTarget` _mesh _returnvalue_2 1.0 true)
          (else
            (`SkeletalMeshComponent.SetMorphTarget` _mesh _returnvalue_2 0.0 true)))))))

(fn `setSpeechDurationList`
  (bind _speechlist (`self.SpeechList`))
  (bind _keys (`BlueprintMapLibrary.Map_Keys` _speechlist))
  (for _array_element _keys
    (`BlueprintMapLibrary.Map_Add` (`self.SpeechDurationList`) _array_element (* (`SoundBase.Duration` (`BlueprintMapLibrary.Map_Find` _speechlist _array_element)) 1000.0))))

(fn `setVisemeMap`
  (params (speech_id :type String))
  (bind (_value _returnvalue) (`BlueprintMapLibrary.Map_Find` (`self.SpeechSyncList`) speech_id))
  (if _returnvalue
    (`|ExecutionSequence`
      (:`then_0`
        (`KismetArrayLibrary.Array_Clear` (`self.VisemeList`)))
      (:`then_2`
        (bind _returnvalue_2 (`LowEntryJsonLibrary.Object_GetJsonArray` _value "VisemeList")
          (:`Success`
            (bind (_element _index) (`/LowEntryJson/Blueprints/LowEntryJsonMacros.JsonArrayForEachLoop` _returnvalue_2)
              (:`LoopBody`
                (bind _returnvalue_3 (`LowEntryJsonLibrary.Value_GetJsonObject` _element)
                  (:`Success`
                    (`|ExecutionSequence`
                      (:`then_0`
                        (bind _returnvalue_4 (`LowEntryJsonLibrary.Object_GetString` _returnvalue_3 "value")))
                      (:`then_1`
                        (bind _returnvalue_5 (`LowEntryJsonLibrary.Object_GetInteger` _returnvalue_3 "time")))
                      (:`then_2`
                        (bind _returnvalue_6 (`LowEntryJsonLibrary.Object_GetString` _returnvalue_3 "type")))
                      (:`then_3`
                        (`KismetArrayLibrary.Array_Insert` (`self.VisemeList`) (make `/Game/ARINBody/Data/VisemeListStruct` _returnvalue_5 _returnvalue_6 _returnvalue_4) _index))))))
              (:`Completed`
                (set `self.VisemeMax` (`KismetArrayLibrary.Array_Length` (`self.VisemeList`)))
                (set `self.VisemeIndex` 0)))))))))

(fn `UserConstructionScript`)