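; Body animation controller that drives the ControllerNum slot of the CH_ARINBody AnimBlueprint's per-controller arrays.
; Tick runs a timed state machine for prep, stroke and relax, writing blend alphas, play rates and state flags, with relative, absolute, periodic and two-part stroke variants.
; Bound AnimBP events interrupt into relax or, for all but one controller number, restore buffered animation.
; DoStroke and DoPrep extend the parent by clearing TurnFlag, which relax sets again.
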(event `self.ReceiveBeginPlay`
  (`|ExecutionSequence`
    (:`then_0`
      (bind _outactors (`GameplayStatics.GetAllActorsOfClass` "/Game/ARINBody/Blueprints/CH_ARINBody.CH_ARINBody_C"))
      (for _array_element _outactors
        (bind _asbp_arinbody_anim_blueprint (cast `/Game/ARINBody/Blueprints/BP_ARINBody_AnimBlueprint` (`SkeletalMeshComponent.GetAnimInstance` (`Character.Mesh` _array_element))))
        (bind _output_get (set `self.AnimBPref` _asbp_arinbody_anim_blueprint))
        (add `/Game/ARINBody/Blueprints/BP_ARINBody_AnimBlueprint.InterruptAnimation` _output_get (delegate `self.InterruptEvent`))
        (if (!= (`self.ControllerNum`) (`KismetMathLibrary.Conv_ByteToInt` (enumliteral `/Game/ARINBody/Data/ControllerNameEnum` "NewEnumerator22")))
          (add `/Game/ARINBody/Blueprints/BP_ARINBody_AnimBlueprint.RestoreAnimation` _output_get (delegate `self.RestoreEvent`)))))
    (:`then_1`
      (bind _outactors_2 (`GameplayStatics.GetAllActorsOfClass` "/Game/ARINBody/Blueprints/BP_JsonDBManager.BP_JsonDBManager_C"))
      (for _array_element_2 _outactors_2
        (set `self.DBManagerRef` _array_element_2)))))

(event `self.InterruptEvent`
  (`self.DoInterruptRelax`))

(event `self.RestoreEvent`
  (bind _animbpref (`self.AnimBPref`))
  (bind _controllernum (`self.ControllerNum`))
  (if (`|GetArrayItem` (`/Game/ARINBody/Blueprints/BP_ARINBody_AnimBlueprint.SavedIsControllerOnArrayInBuffer` _animbpref) _controllernum)
    (`self.DoRestore` (`|GetArrayItem` (`/Game/ARINBody/Blueprints/BP_ARINBody_AnimBlueprint.SavedAnimArrayInBuffer` _animbpref) _controllernum) (`|GetArrayItem` (`/Game/ARINBody/Blueprints/BP_ARINBody_AnimBlueprint.SavedCallArrayInBuffer` _animbpref) _controllernum) (`|GetArrayItem` (`/Game/ARINBody/Blueprints/BP_ARINBody_AnimBlueprint.SavedIsAnimRelArrayInBuffer` _animbpref) _controllernum))
    (else
      (`self.DoRelax` 1.0))))

(event `self.ReceiveTick`
  (params (DeltaSeconds :type "Float (single-precision)"))
  (bind _controllernum (`self.ControllerNum`))
  (bind _controllernum_2 (`self.ControllerNum`))
  (bind _controllerblendalphaarray (`/Game/ARINBody/Blueprints/BP_ARINBody_AnimBlueprint.ControllerBlendAlphaArray` (`self.AnimBPref`)))
  (bind _controllerblendalphaarray_2 (`/Game/ARINBody/Blueprints/BP_ARINBody_AnimBlueprint.ControllerBlendAlphaArray` (`self.AnimBPref`)))
  (if (`self.InterruptFlag`)
    ;[1 1 1] Non Periodic -> Relax
    (`KismetArrayLibrary.Array_Set` _controllerblendalphaarray_2 _controllernum_2 (+ (`|GetArrayItem` (`/Game/ARINBody/Blueprints/BP_ARINBody_AnimBlueprint.ControllerBlendAlphaArray` (`self.AnimBPref`)) (`self.ControllerNum`)) (/ (`GameplayStatics.GetWorldDeltaSeconds`) (`self.RelaxTime`))))
    (if (> (`|GetArrayItem` _controllerblendalphaarray_2 _controllernum_2) 1.0)
      (`KismetArrayLibrary.Array_Set` (`/Game/ARINBody/Blueprints/BP_ARINBody_AnimBlueprint.StateTransitionFlagArray` (`self.AnimBPref`)) (`self.ControllerNum`) 0 true)
      (`KismetArrayLibrary.Array_Set` (`/Game/ARINBody/Blueprints/BP_ARINBody_AnimBlueprint.CurrentStateArray` (`self.AnimBPref`)) (`self.ControllerNum`) 0 true)
      (`KismetArrayLibrary.Array_Set` (`/Game/ARINBody/Blueprints/BP_ARINBody_AnimBlueprint.AnimStartPointArray` (`self.AnimBPref`)) (`self.ControllerNum`))
      (`KismetArrayLibrary.Array_Set` (`/Game/ARINBody/Blueprints/BP_ARINBody_AnimBlueprint.CurAnimStartPointArray` (`self.AnimBPref`)) (`self.ControllerNum`))
      (set `self.IsStroke1Finished` false)
      (set `self.State` 0)
      (`KismetArrayLibrary.Array_Set` (`/Game/ARINBody/Blueprints/BP_ARINBody_AnimBlueprint.CurCallArray` (`self.AnimBPref`)) (`self.ControllerNum`))
      (set `self.TurnFlag` 1)
      (set `self.InterruptFlag` false))
    (else
      (switch `int` (`self.State`)
        (:`1`
          (if (`|GetArrayItem` (`/Game/ARINBody/Blueprints/BP_ARINBody_AnimBlueprint.IsAnimRelArray` (`self.AnimBPref`)) (`self.ControllerNum`))
            ;[1 1 1] Rel No Prepeation, Blend with new  Anim
            (if (`self.IsStrokeSeperated`)
              (if (`self.IsStroke1Finished`)
                (`KismetArrayLibrary.Array_Set` (`/Game/ARINBody/Blueprints/BP_ARINBody_AnimBlueprint.AnimBlendAlphaArray` (`self.AnimBPref`)) (`self.ControllerNum`) 1.0)
                (else
                  (`KismetArrayLibrary.Array_Set` (`/Game/ARINBody/Blueprints/BP_ARINBody_AnimBlueprint.AnimStartPointArray` (`self.AnimBPref`)) (`self.ControllerNum`) :!label _label)
                  (bind _output_get (set `self.PrepTimer` (+ (`self.PrepTimer`) (`GameplayStatics.GetWorldDeltaSeconds`))))
                  (`KismetArrayLibrary.Array_Set` (`/Game/ARINBody/Blueprints/BP_ARINBody_AnimBlueprint.AnimBlendAlphaArray` (`self.AnimBPref`)) (`self.ControllerNum`) (/ _output_get (`self.Preptime`)))))
              (else
                (goto _label)))
            (`KismetArrayLibrary.Array_Set` (`/Game/ARINBody/Blueprints/BP_ARINBody_AnimBlueprint.StateTransitionFlagArray` (`self.AnimBPref`)) (`self.ControllerNum`) 1 true)
            ;[1 1 1] Stroke Rel
            (`KismetArrayLibrary.Array_Set` (`/Game/ARINBody/Blueprints/BP_ARINBody_AnimBlueprint.PlayRateArray` (`self.AnimBPref`)) (`self.ControllerNum`) (`self.PlayRate`) true)
            (bind _output_get_2 (set `self.StrokeTimer` (+ (`self.StrokeTimer`) (`GameplayStatics.GetWorldDeltaSeconds`))))
            (if (>= _output_get_2 (/ (`self.AnimLength`) (`|GetArrayItem` (`/Game/ARINBody/Blueprints/BP_ARINBody_AnimBlueprint.PlayRateArray` (`self.AnimBPref`)) (`self.ControllerNum`))))
              (`KismetArrayLibrary.Array_Set` (`/Game/ARINBody/Blueprints/BP_ARINBody_AnimBlueprint.CurAnimArray` (`self.AnimBPref`)) (`self.ControllerNum`) (`|GetArrayItem` (`/Game/ARINBody/Blueprints/BP_ARINBody_AnimBlueprint.NewAnimArray` (`self.AnimBPref`)) (`self.ControllerNum`)) true)
              (if (`self.IsStrokeSeperated`)
                (if (`self.IsStroke1Finished`)
                  (set `self.IsStroke1Finished` false)
                  (`KismetArrayLibrary.Array_Set` (`/Game/ARINBody/Blueprints/BP_ARINBody_AnimBlueprint.CurAnimStartPointArray` (`self.AnimBPref`)) (`self.ControllerNum`) 100.0 :!label _label_2)
                  (`KismetArrayLibrary.Array_Set` (`/Game/ARINBody/Blueprints/BP_ARINBody_AnimBlueprint.CurCallArray` (`self.AnimBPref`)) (`self.ControllerNum`) 3)
                  (else
                    (set `self.IsStroke1Finished` true)
                    (`KismetArrayLibrary.Array_Set` (`/Game/ARINBody/Blueprints/BP_ARINBody_AnimBlueprint.CurAnimStartPointArray` (`self.AnimBPref`)) (`self.ControllerNum`) (`self.AnimLength`))
                    (`KismetArrayLibrary.Array_Set` (`/Game/ARINBody/Blueprints/BP_ARINBody_AnimBlueprint.CurCallArray` (`self.AnimBPref`)) (`self.ControllerNum`) 2)))
                (else
                  (goto _label_2)))
              (set `self.State` 0)
              (`KismetArrayLibrary.Array_Set` (`/Game/ARINBody/Blueprints/BP_ARINBody_AnimBlueprint.StateTransitionFlagArray` (`self.AnimBPref`)) (`self.ControllerNum`) 2 true)
              (`self.InitializeVariable`)
              (if (`self.IsPeriodic`)
                (if (`self.IsStrokeSeperated`)
                  (if (`self.IsStroke1Finished`)
                    (`KismetArrayLibrary.Array_Set` (`/Game/ARINBody/Blueprints/BP_ARINBody_AnimBlueprint.CurrentStateArray` (`self.AnimBPref`)) (`self.ControllerNum`) 2 true :!label _label_3)
                    (else
                      (set `self.State` 2 :!label _label_4)))
                  (else
                    (goto _label_4)))
                (else
                  (goto _label_3))))
            (else
              ;[1 1 1] Stroke Abs
              (if (`self.IsStrokeSeperated`)
                (if (not (`self.IsStroke1Finished`))
                  (`KismetArrayLibrary.Array_Set` (`/Game/ARINBody/Blueprints/BP_ARINBody_AnimBlueprint.AnimStartPointArray` (`self.AnimBPref`)) (`self.ControllerNum`) :!label _label_5))
                (else
                  (goto _label_5)))
              (`KismetArrayLibrary.Array_Set` (`/Game/ARINBody/Blueprints/BP_ARINBody_AnimBlueprint.AnimBlendAlphaArray` (`self.AnimBPref`)) (`self.ControllerNum`) 1.0)
              (`KismetArrayLibrary.Array_Set` (`/Game/ARINBody/Blueprints/BP_ARINBody_AnimBlueprint.PlayRateArray` (`self.AnimBPref`)) (`self.ControllerNum`) (`self.PlayRate`) true)
              (`KismetArrayLibrary.Array_Set` (`/Game/ARINBody/Blueprints/BP_ARINBody_AnimBlueprint.StateTransitionFlagArray` (`self.AnimBPref`)) (`self.ControllerNum`) 1)
              (bind _output_get_3 (set `self.StrokeTimer` (+ (`self.StrokeTimer`) (`GameplayStatics.GetWorldDeltaSeconds`))))
              (if (>= _output_get_3 (/ (`self.AnimLength`) (`|GetArrayItem` (`/Game/ARINBody/Blueprints/BP_ARINBody_AnimBlueprint.PlayRateArray` (`self.AnimBPref`)) (`self.ControllerNum`))))
                (`KismetArrayLibrary.Array_Set` (`/Game/ARINBody/Blueprints/BP_ARINBody_AnimBlueprint.CurAnimArray` (`self.AnimBPref`)) (`self.ControllerNum`) (`|GetArrayItem` (`/Game/ARINBody/Blueprints/BP_ARINBody_AnimBlueprint.NewAnimArray` (`self.AnimBPref`)) (`self.ControllerNum`)) true)
                (set `self.State` 0)
                (`KismetArrayLibrary.Array_Set` (`/Game/ARINBody/Blueprints/BP_ARINBody_AnimBlueprint.StateTransitionFlagArray` (`self.AnimBPref`)) (`self.ControllerNum`) 2 true)
                (if (`self.IsStrokeSeperated`)
                  (if (`self.IsStroke1Finished`)
                    (set `self.IsStroke1Finished` false)
                    (`KismetArrayLibrary.Array_Set` (`/Game/ARINBody/Blueprints/BP_ARINBody_AnimBlueprint.CurAnimStartPointArray` (`self.AnimBPref`)) (`self.ControllerNum`) 100.0 :!label _label_6)
                    (`KismetArrayLibrary.Array_Set` (`/Game/ARINBody/Blueprints/BP_ARINBody_AnimBlueprint.CurCallArray` (`self.AnimBPref`)) (`self.ControllerNum`) 3)
                    (else
                      (set `self.IsStroke1Finished` true)
                      (`KismetArrayLibrary.Array_Set` (`/Game/ARINBody/Blueprints/BP_ARINBody_AnimBlueprint.CurAnimStartPointArray` (`self.AnimBPref`)) (`self.ControllerNum`) (`self.AnimLength`))
                      (`KismetArrayLibrary.Array_Set` (`/Game/ARINBody/Blueprints/BP_ARINBody_AnimBlueprint.CurCallArray` (`self.AnimBPref`)) (`self.ControllerNum`) 2)))
                  (else
                    (goto _label_6)))
                (`KismetArrayLibrary.Array_Set` (`/Game/ARINBody/Blueprints/BP_ARINBody_AnimBlueprint.CurBodyPartsArray` (`self.AnimBPref`)) (`self.ControllerNum`) (`|GetArrayItem` (`/Game/ARINBody/Blueprints/BP_ARINBody_AnimBlueprint.BonePartsArray` (`self.AnimBPref`)) (`self.ControllerNum`)))
                (`self.InitializeVariable`)
                (`KismetArrayLibrary.Array_Set` (`/Game/ARINBody/Blueprints/BP_ARINBody_AnimBlueprint.CurrentStateArray` (`self.AnimBPref`)) (`self.ControllerNum`) 1 true)))))
        (:`2`
          (if (`self.IsPeriodic`)
            (if (`|GetArrayItem` (`/Game/ARINBody/Blueprints/BP_ARINBody_AnimBlueprint.IsAnimRelArray` (`self.AnimBPref`)) (`self.ControllerNum`))
              ;[1 1 1] Periodic -> Relax
              (`KismetArrayLibrary.Array_Set` (`/Game/ARINBody/Blueprints/BP_ARINBody_AnimBlueprint.ControllerBlendAlphaArray` (`self.AnimBPref`)) (`self.ControllerNum`) 1.0)
              (`KismetArrayLibrary.Array_Set` (`/Game/ARINBody/Blueprints/BP_ARINBody_AnimBlueprint.CurrentStateArray` (`self.AnimBPref`)) (`self.ControllerNum`) 0 true)
              (`KismetArrayLibrary.Array_Set` (`/Game/ARINBody/Blueprints/BP_ARINBody_AnimBlueprint.StateTransitionFlagArray` (`self.AnimBPref`)) (`self.ControllerNum`) 0 true)
              (`KismetArrayLibrary.Array_Set` (`/Game/ARINBody/Blueprints/BP_ARINBody_AnimBlueprint.AnimStartPointArray` (`self.AnimBPref`)))
              (`KismetArrayLibrary.Array_Set` (`/Game/ARINBody/Blueprints/BP_ARINBody_AnimBlueprint.CurAnimStartPointArray` (`self.AnimBPref`)) (`self.ControllerNum`))
              (set `self.IsStroke1Finished` false)
              (set `self.State` 0)
              (`KismetArrayLibrary.Array_Set` (`/Game/ARINBody/Blueprints/BP_ARINBody_AnimBlueprint.CurCallArray` (`self.AnimBPref`)) (`self.ControllerNum`))
              (set `self.TurnFlag` 1)
              (else
                ;[1 1 1] Non Periodic -> Relax
                (bind _output_get_4 (set `self.RelaxTimer` (+ (`self.RelaxTimer`) (`GameplayStatics.GetWorldDeltaSeconds`)) :!label _label_7))
                (`KismetArrayLibrary.Array_Set` _controllerblendalphaarray _controllernum (/ _output_get_4 (`self.RelaxTime`)))
                (if (> (`|GetArrayItem` _controllerblendalphaarray _controllernum) 1.0)
                  (`KismetArrayLibrary.Array_Set` (`/Game/ARINBody/Blueprints/BP_ARINBody_AnimBlueprint.StateTransitionFlagArray` (`self.AnimBPref`)) (`self.ControllerNum`) 0 true)
                  (`KismetArrayLibrary.Array_Set` (`/Game/ARINBody/Blueprints/BP_ARINBody_AnimBlueprint.CurrentStateArray` (`self.AnimBPref`)) (`self.ControllerNum`) 0 true)
                  (`KismetArrayLibrary.Array_Set` (`/Game/ARINBody/Blueprints/BP_ARINBody_AnimBlueprint.AnimStartPointArray` (`self.AnimBPref`)) (`self.ControllerNum`))
                  (`KismetArrayLibrary.Array_Set` (`/Game/ARINBody/Blueprints/BP_ARINBody_AnimBlueprint.CurAnimStartPointArray` (`self.AnimBPref`)) (`self.ControllerNum`))
                  (set `self.IsStroke1Finished` false)
                  (set `self.State` 0)
                  (`KismetArrayLibrary.Array_Set` (`/Game/ARINBody/Blueprints/BP_ARINBody_AnimBlueprint.CurCallArray` (`self.AnimBPref`)) (`self.ControllerNum`))
                  (set `self.TurnFlag` 1))))
            (else
              (goto _label_7))))
        (:`3`
          ;[1 1 1] Abs Preperation
          (`KismetArrayLibrary.Array_Set` (`/Game/ARINBody/Blueprints/BP_ARINBody_AnimBlueprint.StateTransitionFlagArray` (`self.AnimBPref`)) (`self.ControllerNum`) 1 true)
          (bind _output_get_5 (set `self.PrepTimer` (+ (`self.PrepTimer`) (`GameplayStatics.GetWorldDeltaSeconds`))))
          (`KismetArrayLibrary.Array_Set` (`/Game/ARINBody/Blueprints/BP_ARINBody_AnimBlueprint.AnimBlendAlphaArray` (`self.AnimBPref`)) (`self.ControllerNum`) (/ _output_get_5 (`self.Preptime`)))
          (if (> (`|GetArrayItem` (`/Game/ARINBody/Blueprints/BP_ARINBody_AnimBlueprint.AnimBlendAlphaArray` (`self.AnimBPref`)) (`self.ControllerNum`)) 1.0)
            (`KismetArrayLibrary.Array_Set` (`/Game/ARINBody/Blueprints/BP_ARINBody_AnimBlueprint.CurAnimArray` (`self.AnimBPref`)) (`self.ControllerNum`) (`|GetArrayItem` (`/Game/ARINBody/Blueprints/BP_ARINBody_AnimBlueprint.NewAnimArray` (`self.AnimBPref`)) (`self.ControllerNum`)) true)
            (set `self.State` 0)
            (`KismetArrayLibrary.Array_Set` (`/Game/ARINBody/Blueprints/BP_ARINBody_AnimBlueprint.StateTransitionFlagArray` (`self.AnimBPref`)) (`self.ControllerNum`) 2 true)
            (`KismetArrayLibrary.Array_Set` (`/Game/ARINBody/Blueprints/BP_ARINBody_AnimBlueprint.CurAnimStartPointArray` (`self.AnimBPref`)) (`self.ControllerNum`) (`|GetArrayItem` (`/Game/ARINBody/Blueprints/BP_ARINBody_AnimBlueprint.AnimStartPointArray` (`self.AnimBPref`)) (`self.ControllerNum`)))
            (`KismetArrayLibrary.Array_Set` (`/Game/ARINBody/Blueprints/BP_ARINBody_AnimBlueprint.CurBodyPartsArray` (`self.AnimBPref`)) (`self.ControllerNum`) (`|GetArrayItem` (`/Game/ARINBody/Blueprints/BP_ARINBody_AnimBlueprint.BonePartsArray` (`self.AnimBPref`)) (`self.ControllerNum`)))
            (`self.InitializeVariable`)
            (if (`|GetArrayItem` (`/Game/ARINBody/Blueprints/BP_ARINBody_AnimBlueprint.IsAnimRelArray` (`self.AnimBPref`)) (`self.ControllerNum`))
              (`KismetArrayLibrary.Array_Set` (`/Game/ARINBody/Blueprints/BP_ARINBody_AnimBlueprint.CurrentStateArray` (`self.AnimBPref`)) (`self.ControllerNum`) 2 true)
              (else
                (`KismetArrayLibrary.Array_Set` (`/Game/ARINBody/Blueprints/BP_ARINBody_AnimBlueprint.CurrentStateArray` (`self.AnimBPref`)) (`self.ControllerNum`) 1 true)))
            (if (`self.IsPose`)
              (`KismetArrayLibrary.Array_Set` (`/Game/ARINBody/Blueprints/BP_ARINBody_AnimBlueprint.CurCallArray` (`self.AnimBPref`)) (`self.ControllerNum`) 3)
              (elif (`self.IsStroke1Finished`)
                (`KismetArrayLibrary.Array_Set` (`/Game/ARINBody/Blueprints/BP_ARINBody_AnimBlueprint.CurCallArray` (`self.AnimBPref`)) (`self.ControllerNum`) 2)
                (else
                  (`KismetArrayLibrary.Array_Set` (`/Game/ARINBody/Blueprints/BP_ARINBody_AnimBlueprint.CurCallArray` (`self.AnimBPref`)) (`self.ControllerNum`) 1))))))))))

(fn `DoPrep`
  (params (AnimPath :type Name) (PreperationTime :type "Float (double-precision)") (IsPose :type Integer) (IsRelative :type Integer) (IsPeriodic :type Integer))
  (`parent.DoPrep` AnimPath PreperationTime IsPose IsRelative IsPeriodic)
  (set `self.TurnFlag` 0)
  (return))

(fn `DoStroke`
  (params (PathName :type Name) (StrokeTime :type "Float (double-precision)") (IsPose :type Integer) (IsRelative :type Integer) (IsPeriodic :type Integer))
  (`parent.DoStroke` PathName StrokeTime IsPose IsRelative IsPeriodic)
  (set `self.TurnFlag` 0)
  (return))

(fn `UserConstructionScript`
  (`parent.UserConstructionScript`))