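; VideoPlayActor plays local video files through a media player, with Play, Pause and Stop controls.
; On BeginPlay it links the media texture and sound to the player, feeding the texture into a half-opacity dynamic material and the ContetentsImage brush.
; Play opens a file URL for a new file name or resumes the current one, while Stop closes the media and clears the name.
; A failed media open prints an on-screen message.
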(event `self.ReceiveBeginPlay`
  (bind _mediatextureref (`self.MediaTextureRef`))
  (bind _contetentsimage (`self.ContetentsImage`))
  (bind (_brush_imagesize _brush_margin _brush_tintcolor _brush_resourceobject _brush_drawas _brush_tiling _brush_mirroring) (break `SlateBrush` (`Image.Brush` _contetentsimage)))
  (bind _returnvalue (`KismetMaterialLibrary.CreateDynamicMaterialInstance` "/Game/ARINBody/Data/VideoMaterial.VideoMaterial"))
  (set `self.MediaMaterial` _returnvalue)
  (set `Texture.CompressionSettings` "TC_Default" _mediatextureref)
  (set `Texture.SRGB` true _mediatextureref)
  (`MaterialInstanceDynamic.SetTextureParameterValue` (`self.MediaMaterial`) "Texture" (`self.MediaTextureRef`))
  (`MediaTexture.SetMediaPlayer` (`self.MediaTextureRef`) (`self.MediaPlayerRef`))
  (`MaterialInstanceDynamic.SetScalarParameterValue` (`self.MediaMaterial`) "Opacity" 0.5)
  (`MediaSoundComponent.SetMediaPlayer` (`self.MediaSound`) (`self.MediaPlayerRef`))
  (`Image.SetBrush` _contetentsimage (make `SlateBrush` _brush_imagesize _brush_margin _brush_tintcolor (`self.MediaTextureRef`) _brush_drawas _brush_tiling _brush_mirroring)))

(event `self.MediaPlayerRef.OnMediaOpenFailed`
  (params (FailedUrl :type String))
  (`KismetSystemLibrary.PrintString` "Fail Video" true true (struct :`G` 0.66 :`B` 1.0 :`A` 1.0) 10.0))

(fn `Pause`
  (`MediaPlayer.Pause` (`self.MediaPlayerRef`)))

(fn `Play`
  (params (FileName :type String))
  (bind _mediaplayerref (`self.MediaPlayerRef`))
  (if (`KismetStringLibrary.EqualEqual_StrStr` FileName (`self.FileName`))
    (`MediaPlayer.Play` _mediaplayerref)
    (else
      (bind _output_get (set `self.FileName` FileName))
      (`MediaPlayer.OpenUrl` _mediaplayerref (`KismetStringLibrary.Concat_StrStr` "file://" _output_get))
      (`MediaPlayer.Play` _mediaplayerref))))

(fn `Stop`
  (`MediaPlayer.Close` (`self.MediaPlayerRef`))
  (set `self.FileName` ""))

(fn `UserConstructionScript`)