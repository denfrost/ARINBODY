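; Controller that turns the ARINBody character in place to face a target looked up by ID in its object array.
; BeginPlay caches the character, its anim blueprint and the reach controller.
; TurnControlCall computes the shortest yaw, derives duration from angle when negative, feeds angle and play rate to animation, and can interrupt reach relax.
; Tick rotates the actor and updates blend alpha until the timer clears the turn flag.
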(event `self.ReceiveBeginPlay`
  ;[1 1 1] BeginPlayEvent(Initialize ARINBodyAnimBP Reference)
  (`|ExecutionSequence`
    (:`then_0`
      (bind _outactors (`GameplayStatics.GetAllActorsOfClass` "/Game/ARINBody/Blueprints/CH_ARINBody.CH_ARINBody_C"))
      (for _array_element _outactors
        (bind _asbp_arinbody_anim_blueprint (cast `/Game/ARINBody/Blueprints/BP_ARINBody_AnimBlueprint` (`SkeletalMeshComponent.GetAnimInstance` (`Character.Mesh` _array_element))))
        (set `self.AnimBPref` _asbp_arinbody_anim_blueprint)))
    (:`then_1`
      (bind _outactors_2 (`GameplayStatics.GetAllActorsOfClass` "/Game/ARINBody/Blueprints/CH_ARINBody.CH_ARINBody_C"))
      (for _array_element_2 _outactors_2
        (set `self.CharacterRef` _array_element_2)))
    (:`then_2`
      (bind _outactors_3 (`GameplayStatics.GetAllActorsOfClass` "/Game/ARINBody/Blueprints/BP_ReachController.BP_ReachController_C"))
      (for _array_element_3 _outactors_3
        (set `self.ReachControllerRef` _array_element_3)))))

(event `self.ReceiveTick`
  (params (DeltaSeconds :type "Float (single-precision)"))
  (bind _animblendalphaarray (`/Game/ARINBody/Blueprints/BP_ARINBody_AnimBlueprint.AnimBlendAlphaArray` (`self.AnimBPref`)))
  (if (`/Game/ARINBody/Blueprints/BP_ARINBody_AnimBlueprint.TurnFlag` (`self.AnimBPref`))
    ;[1 1 1] Tick Event(Run Turn Animation Timer and Call Turn Anim Finish Event)
    (bind _output_get (set `self.TurnTimer` (+ (`GameplayStatics.GetWorldDeltaSeconds`) (`self.TurnTimer`))))
    (`self.K2_AddActorWorldRotation` (`self.CharacterRef`) (`KismetMathLibrary.MakeRotator` 0.0 0.0 (* (/ DeltaSeconds (`self.TurnTime`)) (`self.TurnAngle`))) false false)
    (bind _returnvalue (* _output_get 0.0))
    (if (< _returnvalue 0.95)
      (`KismetArrayLibrary.Array_Set` _animblendalphaarray (`self.ControllerNum`))
      (else
        (`KismetArrayLibrary.Array_Set` _animblendalphaarray (`self.ControllerNum`) (* (- _returnvalue 0.95) 20.0))))
    (if (> _output_get (/ 1.0 (`|GetArrayItem` (`/Game/ARINBody/Blueprints/BP_ARINBody_AnimBlueprint.PlayRateArray` (`self.AnimBPref`)) (`self.ControllerNum`))))
      (set `self.TurnTimer` 0.0)
      (set `/Game/ARINBody/Blueprints/BP_ARINBody_AnimBlueprint.TurnFlag` false (`self.AnimBPref`)))))

(fn `SetPosition`
  (params (ObjectArrayIdx :type Integer) (Position :type "Vector Structure"))
  (bind _characterref (`self.CharacterRef`))
  (if (== ObjectArrayIdx -1)
    (`/Game/ARINBody/Blueprints/CH_ARINBody.SetPositionofIndex` _characterref (`self.ControllerNum`) Position)
    (else
      (`/Game/ARINBody/Blueprints/CH_ARINBody.SetPositionofIndex` _characterref ObjectArrayIdx Position))))

(fn `TurnControlCall`
  (params (ObjectID :type Integer) (TurnTime :type "Float (double-precision)"))
  (bind (_returnvalue_roll _returnvalue_pitch _returnvalue_yaw) (`KismetMathLibrary.BreakRotator` (`SceneComponent.K2_GetComponentRotation` (`Actor.RootComponent` (`self.CharacterRef`)))))
  (bind _returnvalue (- 180.0 (- (`KismetMathLibrary.Abs` (`self.TurnAngle`)) 180.0)))
  (bind (_returnvalue_roll_2 _returnvalue_pitch_2 _returnvalue_yaw_2) (`KismetMathLibrary.BreakRotator` (`KismetMathLibrary.FindLookAtRotation` (`SceneComponent.K2_GetComponentLocation` (`Actor.RootComponent` (`self.CharacterRef`))) (`BlueprintMapLibrary.Map_Find` (`/Game/ARINBody/Blueprints/CH_ARINBody.ObjectArray` (`self.CharacterRef`)) (`self.ObjectID`)))))
  (if (== ObjectID -1)
    (set `self.ObjectID` (`self.ControllerNum`))
    (else
      (set `self.ObjectID` ObjectID)))
  (if (not (`.ReturnValue` (`BlueprintMapLibrary.Map_Find` (`/Game/ARINBody/Blueprints/CH_ARINBody.ObjectArray` (`self.CharacterRef`)) (`self.ObjectID`))))
    (set `self.ObjectID` (`self.ControllerNum`)))
  (if (not (`/Game/ARINBody/Blueprints/BP_ARINBody_AnimBlueprint.TurnFlag` (`self.AnimBPref`)))
    (bind _output_get (set `self.TurnTime` TurnTime))
    (set `self.TurnAngle` (- _returnvalue_yaw_2 _returnvalue_yaw))
    (if (< _output_get 0.0)
      ;[1 1 1] Set Anim Time
      (set `self.TurnTime` (`KismetMathLibrary.FClamp` (/ (`KismetMathLibrary.Abs` (`self.TurnAngle`)) 90.0) 0.7 3.0)))
    ;[1 1 1] Set Turn Angle Under 180
    (if (> (`KismetMathLibrary.Abs` (`self.TurnAngle`)) 180.0)
      (if (> (`self.TurnAngle`) 0.0)
        (set `self.TurnAngle` (* _returnvalue -1.0))
        (else
          (set `self.TurnAngle` _returnvalue))))
    ;[1 1 1] Set Variables and Start Turn
    (set `/Game/ARINBody/Blueprints/BP_ARINBody_AnimBlueprint.TurnAngle` (`self.TurnAngle`) (`self.AnimBPref`))
    (`KismetArrayLibrary.Array_Set` (`/Game/ARINBody/Blueprints/BP_ARINBody_AnimBlueprint.PlayRateArray` (`self.AnimBPref`)) (`self.ControllerNum`) (/ 1.0 (`self.TurnTime`)))
    (set `/Game/ARINBody/Blueprints/BP_ARINBody_AnimBlueprint.TurnFlag` true (`self.AnimBPref`))
    (set `self.TurnTimer` 0.0)
    (set `self.TurnFlag` 0)
    (set `self.GazeUpperFlag` 0)
    (set `self.GazeFlag` 0)
    (if (<= (`|GetArrayItem` (`/Game/ARINBody/Blueprints/BP_ARINBody_AnimBlueprint.ControllerBlendAlphaArray` (`self.AnimBPref`)) (`KismetMathLibrary.Conv_ByteToInt` (enumliteral `/Game/ARINBody/Data/ControllerNameEnum` "NewEnumerator11"))) 0.0)
      (`/Game/ARINBody/Blueprints/BP_ReachController.InterruptRelax` (`self.ReachControllerRef`)))))

(fn `UserConstructionScript`)