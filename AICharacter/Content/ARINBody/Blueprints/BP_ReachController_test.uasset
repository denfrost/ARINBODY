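; Test controller that drives right-arm reaching on the ARIN body character toward a target looked up by object ID.
; BeginPlay caches the character, its AnimBP and DB manager, and attaches a BoneRotationChecker to the base bone socket as a rotation reference.
; Each Tick computes clavicle-to-target look-at rotation relative to that reference, flips pitch, wraps angles near ±180 and interpolates.
; The results feed the AnimBP's ReachRotator and ReachTarget.
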(event `self.ReceiveBeginPlay`
  (`|ExecutionSequence`
    (:`then_0`
      (bind _outactors (`GameplayStatics.GetAllActorsOfClass` "/Game/ARINBody/Blueprints/CH_ARINBody.CH_ARINBody_C"))
      (for _array_element _outactors
        (bind _mesh (`Character.Mesh` _array_element))
        (bind _asbp_arinbody_anim_blueprint (cast `/Game/ARINBody/Blueprints/BP_ARINBody_AnimBlueprint` (`SkeletalMeshComponent.GetAnimInstance` _mesh)))
        (set `self.AnimBPref` _asbp_arinbody_anim_blueprint)
        (set `self.ControllerNum` (`KismetMathLibrary.Conv_ByteToInt` (enumliteral `/Game/ARINBody/Data/ControllerNameEnum` "NewEnumerator11")))
        (bind _returnvalue (`|SpawnActorFromClass` "/Game/ARINBody/Blueprints/BoneRotationChecker.BoneRotationChecker_C" (`KismetMathLibrary.MakeTransform` (0.0 0.0 0.0)) "AlwaysSpawn" "OverrideRootScale" null null))
        (set `self.BaseBoneRotationChecker` _returnvalue)
        (`self.K2_AttachToComponent` _returnvalue _mesh (`self.BaseBoneSocket`) "KeepWorld" "KeepWorld" "KeepWorld" true)))
    (:`then_1`
      (bind _outactors_2 (`GameplayStatics.GetAllActorsOfClass` "/Game/ARINBody/Blueprints/BP_DBManager.BP_DBManager_C"))
      (for _array_element_2 _outactors_2
        (set `self.DBManagerRef` _array_element_2)))
    (:`then_2`
      (bind _outactors_3 (`GameplayStatics.GetAllActorsOfClass` "/Game/ARINBody/Blueprints/CH_ARINBody.CH_ARINBody_C"))
      (for _array_element_3 _outactors_3
        (set `self.CharactorRef` _array_element_3)))))

(event `self.ReceiveTick`
  (params (DeltaSeconds :type "Float (single-precision)"))
  (bind _output_get (set `self.LookTarget` (`BlueprintMapLibrary.Map_Find` (`/Game/ARINBody/Blueprints/CH_ARINBody.ObjectArray` (`self.CharactorRef`)) (`self.LookatObjectID`))))
  (bind _outlookattransform (`self.CalculateReachRotations` (`Character.Mesh` (`self.CharactorRef`)) "Bip-R-Clavicle" _output_get (`/Game/ARINBody/Blueprints/BP_ARINBody_AnimBlueprint.ReachRotator` (`self.AnimBPref`))))
  (set `/Game/ARINBody/Blueprints/BP_ARINBody_AnimBlueprint.ReachTarget` _outlookattransform (`self.AnimBPref`)))

(fn `CalculateReachRotations`
  (params (CharacterMesh :type "SkeletalMeshComponent Object Reference") (SorceBone :type Name) (LookatTarget :type "Vector Structure") (InLookAtRotation :type "Rotator Structure"))
  (returns (OutLookAtTransform :type "Transform Structure"))
  (bind _returnvalue (`SceneComponent.GetSocketLocation` CharacterMesh SorceBone))
  (bind _returnvalue_2 (`SceneComponent.K2_GetComponentRotation` (`Actor.RootComponent` (`self.BaseBoneRotationChecker`))))
  (set `self.NewVar_0` _returnvalue)
  (set `self.NewVar_1` _returnvalue_2)
  (bind _outrotator (`self.RemapReachRotator` (`KismetMathLibrary.MakeRotator` (- (.roll (`KismetMathLibrary.FindLookAtRotation` _returnvalue LookatTarget)) (.roll _returnvalue_2)) (* (- (.pitch (`KismetMathLibrary.FindLookAtRotation` _returnvalue LookatTarget)) (.pitch _returnvalue_2)) -1.0) (- (.yaw (`KismetMathLibrary.FindLookAtRotation` _returnvalue LookatTarget)) (.yaw _returnvalue_2)))))
  (bind _output_get (set `self.RawLookatRotation` _outrotator))
  (bind _output_get_2 (set `self.NewLookAtRotation` (`KismetMathLibrary.RInterpTo` InLookAtRotation _output_get (`GameplayStatics.GetWorldDeltaSeconds`) 4.0)))
  (set `/Game/ARINBody/Blueprints/BP_ARINBody_AnimBlueprint.ReachRotator` _output_get_2 (`self.AnimBPref`))
  (return (`KismetMathLibrary.MakeTransform` LookatTarget (`self.NewLookAtRotation`))))

(fn `RemapReachRotator`
  (params (InRotator :type "Rotator Structure"))
  (returns (OutRotator :type "Rotator Structure"))
  (bind _roll (.roll InRotator))
  (bind _pitch (.pitch InRotator))
  (bind _yaw (.yaw InRotator))
  (bind _returnvalue (`KismetMathLibrary.SelectFloat` (- _roll 360.0) _roll (> _roll 179.0)))
  (bind _returnvalue_2 (`KismetMathLibrary.SelectFloat` (- _pitch 360.0) _pitch (> _pitch 179.0)))
  (bind _returnvalue_3 (`KismetMathLibrary.SelectFloat` (- _yaw 360.0) _yaw (> _yaw 179.0)))
  (return (`KismetMathLibrary.MakeRotator` (`KismetMathLibrary.SelectFloat` (+ _returnvalue 360.0) _returnvalue (< _returnvalue -179.0)) (`KismetMathLibrary.SelectFloat` (+ _returnvalue_2 360.0) _returnvalue_2 (< _returnvalue_2 -179.0)) (`KismetMathLibrary.SelectFloat` (+ _returnvalue_3 360.0) _returnvalue_3 (< _returnvalue_3 -179.0)))))

(fn `UserConstructionScript`)