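; BP_EyeController is an early, unfinished controller for eye direction on an ARIN body character.
; InitEyeController stores the character reference and zeroes the default, previous and target directions.
; PlayAnimation only records the requested direction as the target and prints a debug "Hello".
; No event drives interpolation, and an unconnected SetMorphTarget call on the player mesh never runs, so the eyes are not animated here.
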(fn `InitEyeController`
  (params (ARINBodyCharaceter :type "/Game/ARINBody/Blueprints/CH_ARINBody Object Reference"))
  (set `self.ARINBodyCharacterRef` ARINBodyCharaceter)
  (set `self.DefaultDirection` (0.0 0.0 0.0))
  (set `self.PrevDirection` (`self.DefaultDirection`))
  (set `self.TargetDirection` (`self.DefaultDirection`)))

(fn `PlayAnimation`
  (params (direction :type "Vector Structure"))
  (set `self.TargetDirection` direction)
  (`KismetSystemLibrary.PrintString` "Hello"))

(fn `UserConstructionScript`)