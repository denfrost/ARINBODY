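; Database manager Blueprint that gives access to two SQLite databases, one for motion data and one for sound.
; Init functions create a connector for each and open files under the game content directory, printing the result.
; Select functions run queries, often built by a string-format helper, and store result sets for typed field getters.
; GetSoundColumnList walks Sound table rows matching a hard-coded Controller filter and returns one column as a list.
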(fn `GenerateQueryString`
  (params (TableName :type String) (FieldName :type String) (QueryData :type String))
  (returns (QueryString :type String))
  (return (`KismetTextLibrary.Conv_TextToString` (`|FormatText` "select * from {0} where {1} = '{2}'" (`KismetTextLibrary.Conv_StringToText` TableName) (`KismetTextLibrary.Conv_StringToText` FieldName) (`KismetTextLibrary.Conv_StringToText` QueryData)))))

(fn `GetFloatField`
  (params (ColumnName :type String))
  (returns (RetrievedOutput :type "Float (double-precision)"))
  (bind _value (`SQLiteResultor.GetFloat` (`self.MotionDBResultor`) ColumnName))
  (return _value))

(fn `GetIntField`
  (params (ColumnName :type String))
  (returns (RetrievedOutput :type Integer))
  (bind _value (`SQLiteResultor.GetInt` (`self.MotionDBResultor`) ColumnName))
  (return _value))

(fn `GetSoundColumnList`
  (params (ColumnName :type String))
  (returns (ColumnList :type "Array of String"))
  (bind _querystring (`self.GenerateQueryString` "Sound" "Controller" "Sound"))
  (bind _numberofrecord (`self.SelectSoundRecord` _querystring))
  (`KismetSystemLibrary.PrintString` (`KismetStringLibrary.Concat_StrStr` "Number of Selected Record in SoundDB: " (`KismetStringLibrary.Conv_IntToString` _numberofrecord)) true true (struct :`R` 1.0 :`G` 0.11875 :`A` 1.0) 10.0)
  (`|ExecutionSequence`
    (:`then_0`
      (`SQLiteResultor.MoveToFirst` (`self.SoundDBResultor`))
      (`KismetArrayLibrary.Array_Clear` (`self.ColumnList`)))
    (:`then_1`
      (while (not (`self.IsAtEnd`))
        (`|ExecutionSequence`
          (:`then_0`
            (bind _value (`SQLiteResultor.GetString` (`self.SoundDBResultor`) ColumnName))
            (`KismetArrayLibrary.Array_Add` (`self.ColumnList`) _value))
          (:`then_1`
            (`SQLiteResultor.MoveToNext` (`self.SoundDBResultor`)))
          (:`then_2`
            (bind _returnvalue (`SQLiteResultor.IsAtEnd` (`self.SoundDBResultor`)))
            (set `self.IsAtEnd` _returnvalue))))
      (return (`self.ColumnList`)))))

(fn `GetSoundStringField`
  (params (ColumnName :type String))
  (returns (RetrievedOutput :type String))
  (bind _value (`SQLiteResultor.GetString` (`self.SoundDBResultor`) ColumnName))
  (return _value))

(fn `GetStringField`
  (params (ColumnName :type String))
  (returns (RetrievedOutput :type String))
  (bind _value (`SQLiteResultor.GetString` (`self.MotionDBResultor`) ColumnName))
  (return _value))

(fn `InitDBConnector`
  (`|ExecutionSequence`
    (:`then_0`
      (bind _newsqliteconnector (`SQLiteBlueprintFunctionLibrary.CreateSQLiteConnector`))
      (set `self.MotionDBConnector` _newsqliteconnector))
    (:`then_1`
      (bind _newsqliteconnector_2 (`SQLiteBlueprintFunctionLibrary.CreateSQLiteConnector`))
      (set `self.SoundDBConnector` _newsqliteconnector_2))))

(fn `InitDBManager`
  (`|ExecutionSequence`
    (:`then_0`
      (`/Engine/EditorBlueprintResources/StandardMacros.IsValid` (`self.MotionDBConnector`)
        (:`Is Valid`
          ;[1 1 1] make path for database file
          (bind _gamecontentdirectory (`SQLiteBlueprintFunctionLibrary.GameContentDir`))
          (bind _combinedpath (`SQLiteBlueprintFunctionLibrary.Combine` _gamecontentdirectory (`self.DBPathFileName`)))
          (bind _fullpath (`SQLiteBlueprintFunctionLibrary.ConvertRelativePathToFull` _combinedpath))
          ;[1 1 1] open database
          (bind _returninfo (`SQLiteConnector.Open` (`self.MotionDBConnector`) _fullpath))
          (bind (_returninfotype _description) (break `SQLiteReturnInfo` _returninfo))
          (`KismetSystemLibrary.PrintString` (`KismetStringLibrary.Concat_StrStr` (`|GetEnumeratorNameAsString` _returninfotype) " : " _description) true true (struct :`G` 0.66 :`B` 1.0 :`A` 1.0) 20.0))))
    (:`then_1`
      (`/Engine/EditorBlueprintResources/StandardMacros.IsValid` (`self.SoundDBConnector`)
        (:`Is Valid`
          ;[1 1 1] make path for database file
          (bind _gamecontentdirectory_2 (`SQLiteBlueprintFunctionLibrary.GameContentDir`))
          (bind _combinedpath_2 (`SQLiteBlueprintFunctionLibrary.Combine` _gamecontentdirectory_2 (`self.SoundDBPathFileName`)))
          (bind _fullpath_2 (`SQLiteBlueprintFunctionLibrary.ConvertRelativePathToFull` _combinedpath_2))
          ;[1 1 1] open database
          (bind _returninfo_2 (`SQLiteConnector.Open` (`self.SoundDBConnector`) _fullpath_2))
          (bind (_returninfotype_2 _description_2) (break `SQLiteReturnInfo` _returninfo_2))
          (`KismetSystemLibrary.PrintString` (`KismetStringLibrary.Concat_StrStr` (`|GetEnumeratorNameAsString` _returninfotype_2) " : " _description_2) true true (struct :`R` 1.0 :`B` 0.460487 :`A` 1.0) 20.0))))))

(fn `SelectRecord`
  (params (QueryString :type String))
  (returns (NumberOfRecord :type Integer))
  (bind _newsqliteresultor (`SQLiteConnector.ExecuteWithRecordSet` (`self.MotionDBConnector`) QueryString))
  (bind _output_get (set `self.MotionDBResultor` _newsqliteresultor))
  (bind _recordcount (`SQLiteResultor.GetRecordCount` _output_get))
  (return _recordcount))

(fn `SelectSoundRecord`
  (params (QueryString :type String))
  (returns (NumberOfRecord :type Integer))
  (bind _newsqliteresultor (`SQLiteConnector.ExecuteWithRecordSet` (`self.SoundDBConnector`) QueryString))
  (bind _output_get (set `self.SoundDBResultor` _newsqliteresultor))
  (bind _recordcount (`SQLiteResultor.GetRecordCount` _output_get))
  (return _recordcount))

(fn `UserConstructionScript`)