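; Blink controller that animates eye blinks and winks on an ARIN body character's mesh through the eyeBlinkLeft and eyeBlinkRight morph targets.
; Tick runs a toggleable idle blink that ramps weights up and down, then picks a randomized delay before the next one.
; CallBlinkAnimation triggers a timed blink, left wink or right wink, split evenly between closing and opening, and resets the idle timers when it finishes.
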(event `self.ReceiveTick`
  (params (DeltaSeconds :type "Float (single-precision)"))
  (`self.PlayIdleBlinkAnimation`)
  (`self.PlayBlinkAnimation`))

(fn `CallBlinkAnimation`
  (params (type :type String) (time :type "Float (double-precision)"))
  (bind _returnvalue (/ time 2.0))
  (`|ExecutionSequence`
    (:`then_0`
      (set `self.TimePlay` 0.0)
      (set `self.TimeRelax` 0.0))
    (:`then_1`
      (set `self.TimePlayMax` _returnvalue)
      (set `self.TimeRelaxMax` _returnvalue))
    (:`then_2`
      (set `self.TypeBlink` type)
      (set `self.bBlinkAnimation` true))))

(fn `CallIdleBlink`
  (params (bPlayAnimation :type Boolean))
  (`|ExecutionSequence`
    (:`then_0`
      (set `self.TimeIdlePlay` 0.0)
      (set `self.TimeIdleRelax` 0.0)
      (set `self.TimeIdleDelay` 0.0))
    (:`then_2`
      (set `self.bIdleBlinkAnimation` bPlayAnimation))))

(fn `IdleBlinkAnimation`
  (bind _output_get (set `self.TimeIdlePlay` (+ (`self.TimeIdlePlay`) (`GameplayStatics.GetWorldDeltaSeconds`))))
  (if (<= _output_get (`self.TimeIdlePlayMax`))
    (`self.SetBlinkTarget` (/ (`self.TimeIdlePlay`) (`self.TimeIdlePlayMax`)))
    (else
      (bind _output_get_2 (set `self.TimeIdleRelax` (+ (`self.TimeIdleRelax`) (`GameplayStatics.GetWorldDeltaSeconds`))))
      (if (<= _output_get_2 (`self.TimeIdleRelaxMax`))
        (`self.SetBlinkTarget` (- 1.0 (/ (`self.TimeIdleRelax`) (`self.TimeIdleRelaxMax`))))
        (else
          (set `self.TimeIdlePlay` 0.0)
          (set `self.TimeIdleDelay` 0.0)
          (set `self.TimeIdleRelax` 0.0)
          (set `self.TimeIdleDelayMax` (`KismetMathLibrary.RandomFloatInRange` 2.5 4.0)))))))

(fn `InitBlinkController`
  (params (ARINBodyCharacter :type "/Game/ARINBody/Blueprints/CH_ARINBody Object Reference") (BlinkStart :type String))
  (`|ExecutionSequence`
    (:`then_0`
      (set `self.ARINBodyCharacterRef` ARINBodyCharacter))
    (:`then_1`
      (if (`KismetStringLibrary.EqualEqual_StrStr` BlinkStart "True")
        (set `self.bIdleBlinkAnimation` true)
        (elif (`KismetStringLibrary.EqualEqual_StrStr` BlinkStart "False")
          (set `self.bIdleBlinkAnimation` false))))))

(fn `PlayBlinkAnimation`
  (if (`self.bBlinkAnimation`)
    (bind _output_get (set `self.TimePlay` (+ (`self.TimePlay`) (`GameplayStatics.GetWorldDeltaSeconds`))))
    (if (<= _output_get (`self.TimePlayMax`))
      (`self.SetBlinkTargetByType` (`self.TypeBlink`) (/ (`self.TimePlay`) (`self.TimePlayMax`)))
      (else
        (bind _output_get_2 (set `self.TimeRelax` (+ (`self.TimeRelax`) (`GameplayStatics.GetWorldDeltaSeconds`))))
        (if (<= _output_get_2 (`self.TimeRelaxMax`))
          (`self.SetBlinkTargetByType` (`self.TypeBlink`) (- 1.0 (/ (`self.TimeRelax`) (`self.TimeRelaxMax`))))
          (else
            (set `self.TimeIdleDelay` 0.0)
            (set `self.TimeIdlePlay` 0.0)
            (set `self.TimeIdleRelax` 0.0)
            (set `self.bBlinkAnimation` false)))))))

(fn `PlayIdleBlinkAnimation`
  (if (`self.bIdleBlinkAnimation`)
    (bind _output_get (set `self.TimeIdleDelay` (+ (`self.TimeIdleDelay`) (`GameplayStatics.GetWorldDeltaSeconds`))))
    (if (> _output_get (`self.TimeIdleDelayMax`))
      (`self.IdleBlinkAnimation`))))

(fn `SetBlinkTarget`
  (params (Weight :type "Float (double-precision)"))
  (`SkeletalMeshComponent.SetMorphTarget` (`Character.Mesh` (`self.ARINBodyCharacterRef`)) "eyeBlinkLeft" Weight true)
  (`SkeletalMeshComponent.SetMorphTarget` (`Character.Mesh` (`self.ARINBodyCharacterRef`)) "eyeBlinkRight" Weight true))

(fn `SetBlinkTargetByType`
  (params (type :type String) (weight :type "Float (double-precision)"))
  (switch `string` type
    (:`Default`
      (`SkeletalMeshComponent.SetMorphTarget` (`Character.Mesh` (`self.ARINBodyCharacterRef`)) "eyeBlinkLeft" weight true :!label _label)
      (`SkeletalMeshComponent.SetMorphTarget` (`Character.Mesh` (`self.ARINBodyCharacterRef`)) "eyeBlinkRight" weight true))
    (:`Blink`
      (goto _label))
    (:`WinkLeft`
      (`SkeletalMeshComponent.SetMorphTarget` (`Character.Mesh` (`self.ARINBodyCharacterRef`)) "eyeBlinkLeft" weight true)
      (`SkeletalMeshComponent.SetMorphTarget` (`Character.Mesh` (`self.ARINBodyCharacterRef`)) "eyeBlinkRight" 0.0 true))
    (:`WinkRight`
      (`SkeletalMeshComponent.SetMorphTarget` (`Character.Mesh` (`self.ARINBodyCharacterRef`)) "eyeBlinkRight" weight true)
      (`SkeletalMeshComponent.SetMorphTarget` (`Character.Mesh` (`self.ARINBodyCharacterRef`)) "eyeBlinkLeft" 0.0 true))))

(fn `UserConstructionScript`)