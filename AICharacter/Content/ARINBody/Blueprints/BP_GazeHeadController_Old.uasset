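; BP_GazeHeadController_Old drives the ARIN body character's head gaze toward objects by feeding yaw and pitch angles to its AnimBlueprint.
; Do functions compute clamped look-at angles for stroke, relax, restore and re-gaze after body turn or upper-gaze changes, then set a state.
; Tick runs that state, interpolating angles and blend alphas at constant speed, using relative angles when the upper-gaze controller is attached, and resets completion flags.
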(event `self.ReceiveBeginPlay`
  ;[1 1 1] BeginPlayEvent(Initialize  Reference)
  (`|ExecutionSequence`
    (:`then_0`
      (bind _outactors (`GameplayStatics.GetAllActorsOfClass` "/Game/ARINBody/Blueprints/CH_ARINBody.CH_ARINBody_C"))
      (for _array_element _outactors
        (bind _asbp_arinbody_anim_blueprint (cast `/Game/ARINBody/Blueprints/BP_ARINBody_AnimBlueprint` (`SkeletalMeshComponent.GetAnimInstance` (`Character.Mesh` _array_element))))
        (set `self.AnimBPref` _asbp_arinbody_anim_blueprint)))
    (:`then_2`
      (bind _outactors_2 (`GameplayStatics.GetAllActorsOfClass` "/Game/ARINBody/Blueprints/CH_ARINBody.CH_ARINBody_C"))
      (for _array_element_2 _outactors_2
        (set `self.CharactorRef` _array_element_2)))
    (:`then_3`
      (set `self.ControllerNum` (`KismetMathLibrary.Conv_ByteToInt` (enumliteral `/Game/ARINBody/Data/ControllerNameEnum` "NewEnumerator13"))))))

(event `self.ReceiveTick`
  (params (DeltaSeconds :type "Float (single-precision)"))
  (bind _animblendalphaarray (`/Game/ARINBody/Blueprints/BP_ARINBody_AnimBlueprint.AnimBlendAlphaArray` (`self.AnimBPref`)))
  (bind _controllerblendalphaarray (`/Game/ARINBody/Blueprints/BP_ARINBody_AnimBlueprint.ControllerBlendAlphaArray` (`self.AnimBPref`)))
  (bind _controllerblendalphaarray_2 (`/Game/ARINBody/Blueprints/BP_ARINBody_AnimBlueprint.ControllerBlendAlphaArray` (`self.AnimBPref`)))
  ;[1 1 1] TickEvent(Interpolation Angle Parameters)
  (switch `int` (`self.State`)
    (:`1`
      ;;[1 1 1] Stroke
      (if (> (`|GetArrayItem` (`/Game/ARINBody/Blueprints/BP_ARINBody_AnimBlueprint.ControllerBlendAlphaArray` (`self.AnimBPref`)) (`self.ControllerNum`)) 0.0)
        (`KismetArrayLibrary.Array_Set` _controllerblendalphaarray_2 (`self.ControllerNum`) (- (`|GetArrayItem` _controllerblendalphaarray_2 (`self.ControllerNum`)) (/ (`GameplayStatics.GetWorldDeltaSeconds`) (`self.StrokeTime`)))))
      (set `/Game/ARINBody/Blueprints/BP_ARINBody_AnimBlueprint.GazeAngleX` (`KismetMathLibrary.FInterpTo_Constant` (`/Game/ARINBody/Blueprints/BP_ARINBody_AnimBlueprint.GazeAngleX` (`self.AnimBPref`)) (`self.TargetAngleX`) (`GameplayStatics.GetWorldDeltaSeconds`) (/ (`KismetMathLibrary.Abs` (- (`self.TargetAngleX`) (`self.CurAngleX`))) (`self.StrokeTime`))) (`self.AnimBPref`))
      (set `/Game/ARINBody/Blueprints/BP_ARINBody_AnimBlueprint.GazeAngleY` (`KismetMathLibrary.FInterpTo_Constant` (`/Game/ARINBody/Blueprints/BP_ARINBody_AnimBlueprint.GazeAngleY` (`self.AnimBPref`)) (`self.TargetAngleY`) (`GameplayStatics.GetWorldDeltaSeconds`) (/ (`KismetMathLibrary.Abs` (- (`self.TargetAngleY`) (`self.CurAngleY`))) (`self.StrokeTime`))) (`self.AnimBPref`))
      (if (and (== (`/Game/ARINBody/Blueprints/BP_ARINBody_AnimBlueprint.GazeAngleX` (`self.AnimBPref`)) (`self.TargetAngleX`)) (== (`/Game/ARINBody/Blueprints/BP_ARINBody_AnimBlueprint.GazeAngleY` (`self.AnimBPref`)) (`self.TargetAngleY`)))
        (set `self.CurAngleX` (`self.TargetAngleX`))
        (set `self.CurAngleY` (`self.TargetAngleY`))
        (set `self.State` 0)
        (set `self.TurnFlag` 1)
        (set `self.GazeUpperFlag` 1)
        (set `self.GazeFlag` 1)))
    (:`2`
      ;;[1 1 1] Relax
      (if (<= (`|GetArrayItem` (`/Game/ARINBody/Blueprints/BP_ARINBody_AnimBlueprint.ControllerBlendAlphaArray` (`self.AnimBPref`)) (`self.ControllerNum`)) 1.0)
        (bind _output_get (set `self.RelaxTimer` (+ (`self.RelaxTimer`) (`GameplayStatics.GetWorldDeltaSeconds`))))
        (`KismetArrayLibrary.Array_Set` (`/Game/ARINBody/Blueprints/BP_ARINBody_AnimBlueprint.ControllerBlendAlphaArray` (`self.AnimBPref`)) (`self.ControllerNum`) (/ _output_get (`self.StrokeTime`)))
        (set `/Game/ARINBody/Blueprints/BP_ARINBody_AnimBlueprint.GazeAngleX` (`KismetMathLibrary.FInterpTo_Constant` (`/Game/ARINBody/Blueprints/BP_ARINBody_AnimBlueprint.GazeAngleX` (`self.AnimBPref`)) (`self.TargetAngleX`) (`GameplayStatics.GetWorldDeltaSeconds`) (/ (`KismetMathLibrary.Abs` (- (`self.TargetAngleX`) (`self.CurAngleX`))) (`self.StrokeTime`))) (`self.AnimBPref`))
        (set `/Game/ARINBody/Blueprints/BP_ARINBody_AnimBlueprint.GazeAngleY` (`KismetMathLibrary.FInterpTo_Constant` (`/Game/ARINBody/Blueprints/BP_ARINBody_AnimBlueprint.GazeAngleY` (`self.AnimBPref`)) (`self.TargetAngleY`) (`GameplayStatics.GetWorldDeltaSeconds`) (/ (`KismetMathLibrary.Abs` (- (`self.TargetAngleY`) (`self.CurAngleY`))) (`self.StrokeTime`))) (`self.AnimBPref`))
        (if (and (== (`/Game/ARINBody/Blueprints/BP_ARINBody_AnimBlueprint.GazeAngleX` (`self.AnimBPref`)) (`self.TargetAngleX`)) (== (`/Game/ARINBody/Blueprints/BP_ARINBody_AnimBlueprint.GazeAngleY` (`self.AnimBPref`)) (`self.TargetAngleY`)))
          (set `self.CurAngleX` (`self.TargetAngleX`))
          (set `self.CurAngleY` (`self.TargetAngleY`))
          (set `self.State` 0)
          (set `self.TurnFlag` 1)
          (set `self.GazeUpperFlag` 1)
          (set `self.GazeFlag` 1)
          (`KismetArrayLibrary.Array_Set` (`/Game/ARINBody/Blueprints/BP_ARINBody_AnimBlueprint.ControllerBlendAlphaArray` (`self.AnimBPref`)) (`self.ControllerNum`) 1.0))))
    (:`3`
      ;;[1 1 1] Upper Re Gaze
      (if (> (`|GetArrayItem` (`/Game/ARINBody/Blueprints/BP_ARINBody_AnimBlueprint.ControllerBlendAlphaArray` (`self.AnimBPref`)) (`self.ControllerNum`)) 0.0)
        (`KismetArrayLibrary.Array_Set` _controllerblendalphaarray (`self.ControllerNum`) (- (`|GetArrayItem` _controllerblendalphaarray (`self.ControllerNum`)) (/ (`GameplayStatics.GetWorldDeltaSeconds`) (`self.StrokeTime`)))))
      (set `/Game/ARINBody/Blueprints/BP_ARINBody_AnimBlueprint.RelGazeAngleX` (`KismetMathLibrary.FInterpTo_Constant` (`/Game/ARINBody/Blueprints/BP_ARINBody_AnimBlueprint.RelGazeAngleX` (`self.AnimBPref`)) (`self.RelTargetAngleX`) (`GameplayStatics.GetWorldDeltaSeconds`) (/ (`KismetMathLibrary.Abs` (- (`self.RelTargetAngleX`) (`self.CurAngleX`))) (`self.StrokeTime`))) (`self.AnimBPref`))
      (set `/Game/ARINBody/Blueprints/BP_ARINBody_AnimBlueprint.RelGazeAngleY` (`KismetMathLibrary.FInterpTo_Constant` (`/Game/ARINBody/Blueprints/BP_ARINBody_AnimBlueprint.RelGazeAngleY` (`self.AnimBPref`)) (`self.RelTargetAngleY`) (`GameplayStatics.GetWorldDeltaSeconds`) (/ (`KismetMathLibrary.Abs` (- (`self.RelTargetAngleY`) (`self.CurAngleY`))) (`self.StrokeTime`))) (`self.AnimBPref`))
      (if (and (== (`/Game/ARINBody/Blueprints/BP_ARINBody_AnimBlueprint.RelGazeAngleX` (`self.AnimBPref`)) (`self.RelTargetAngleX`)) (== (`/Game/ARINBody/Blueprints/BP_ARINBody_AnimBlueprint.RelGazeAngleY` (`self.AnimBPref`)) (`self.RelTargetAngleY`)))
        (set `self.CurAngleX` (`self.RelTargetAngleX`))
        (set `self.CurAngleY` (`self.RelTargetAngleY`))
        (set `self.State` 0)
        (set `self.TurnFlag` 1)
        (set `self.GazeUpperFlag` 1)
        (set `self.GazeFlag` 1)))
    (:`4`
      ;;[1 1 1] UpperGaze Relax
      (`KismetArrayLibrary.Array_Set` _animblendalphaarray (`self.ControllerNum`) (- (`|GetArrayItem` _animblendalphaarray (`self.ControllerNum`)) (/ (`GameplayStatics.GetWorldDeltaSeconds`) (`self.StrokeTime`))))
      (if (<= (`|GetArrayItem` (`/Game/ARINBody/Blueprints/BP_ARINBody_AnimBlueprint.AnimBlendAlphaArray` (`self.AnimBPref`)) (`self.ControllerNum`)) 0.0)
        (set `self.State` 0)
        (set `self.TurnFlag` 1)
        (set `self.GazeUpperFlag` 1)
        (set `self.GazeFlag` 1)))))

(fn `DoRelax`
  (params (RelaxTime :type "Float (double-precision)"))
  (if (<= (`|GetArrayItem` (`/Game/ARINBody/Blueprints/BP_ARINBody_AnimBlueprint.ControllerBlendAlphaArray` (`self.AnimBPref`)) (`self.ControllerNum`)) 0.0)
    (if (== (`self.State`) 0)
      ;[1 1 1] Set Angles and Timers 0.0 and Relax Start
      (set `self.TargetAngleX` 0.0)
      (set `self.TargetAngleY` 0.0)
      (set `self.State` 2)
      (set `self.StrokeTime` RelaxTime)
      (set `self.PrepTimer` 0.0)
      (set `self.RelaxTimer` 0.0)
      ;[1 1 1] Set Anim Time when Input Time is Negative
      (if (< (`self.StrokeTime`) 0.0)
        (set `self.StrokeTime` 1.0)))))

(fn `DoRestore`
  (params (Curx :type "Float (double-precision)") (Cury :type "Float (double-precision)") (ObjectID :type Integer))
  (bind (_returnvalue_roll _returnvalue_pitch _returnvalue_yaw) (`KismetMathLibrary.BreakRotator` (`SceneComponent.K2_GetComponentRotation` (`Actor.RootComponent` (`self.CharactorRef`)))))
  (bind _value (`BlueprintMapLibrary.Map_Find` (`/Game/ARINBody/Blueprints/CH_ARINBody.ObjectArray` (`self.CharactorRef`)) ObjectID))
  (bind _returnvalue (- 180.0 (- (`KismetMathLibrary.Abs` (`self.TargetAngleX`)) 180.0)))
  (bind (_returnvalue_roll_2 _returnvalue_pitch_2 _returnvalue_yaw_2) (`KismetMathLibrary.BreakRotator` (`KismetMathLibrary.FindLookAtRotation` (+ (`SceneComponent.K2_GetComponentLocation` (`Actor.RootComponent` (`self.CharactorRef`))) (0.0 0.0 80.0)) _value)))
  (if (<= (`|GetArrayItem` (`/Game/ARINBody/Blueprints/BP_ARINBody_AnimBlueprint.ControllerBlendAlphaArray` (`self.AnimBPref`)) (`self.ControllerNum`)) 0.0)
    (set `self.TargetPosition` _value)
    ;[1 1 1] Calculate Axis Angle
    (bind _output_get (set `self.TargetAngleX` (- _returnvalue_yaw_2 _returnvalue_yaw)))
    (if (> (`KismetMathLibrary.Abs` (`self.TargetAngleX`)) 180.0)
      (if (> (`self.TargetAngleX`) 0.0)
        (set `self.TargetAngleX` (`KismetMathLibrary.FClamp` (* _returnvalue -1.0) -80.0 80.0))
        (else
          (set `self.TargetAngleX` (`KismetMathLibrary.FClamp` _returnvalue -80.0 80.0))))
      (else
        (set `self.TargetAngleX` (`KismetMathLibrary.FClamp` _output_get -80.0 80.0))))
    (set `self.TargetAngleY` (`KismetMathLibrary.FClamp` _returnvalue_pitch_2 -50.0 60.0))
    ;[1 1 1] Set Anim Time 1.0
    (set `self.StrokeTime` 1.0)
    ;[1 1 1] Set Relative Target Angle
    (set `self.RelTargetAngleX` (`KismetMathLibrary.FClamp` (- (`self.TargetAngleX`) Curx) -80.0 80.0))
    (set `self.RelTargetAngleY` (`KismetMathLibrary.FClamp` (- (`self.TargetAngleY`) Cury) -50.0 60.0))
    ;[1 1 1] Set Relative Start Point
    (set `/Game/ARINBody/Blueprints/BP_ARINBody_AnimBlueprint.RelGazeAngleX` (`self.CurAngleX`) (`self.AnimBPref`))
    (set `/Game/ARINBody/Blueprints/BP_ARINBody_AnimBlueprint.RelGazeAngleY` (`self.CurAngleY`) (`self.AnimBPref`))
    ;[1 1 1] Start Restore Stroke and Set Flags
    (`KismetArrayLibrary.Array_Set` (`/Game/ARINBody/Blueprints/BP_ARINBody_AnimBlueprint.AnimBlendAlphaArray` (`self.AnimBPref`)) (`self.ControllerNum`) 1.0)
    (set `self.State` 3)
    (set `self.TurnFlag` 0)
    (set `self.GazeUpperFlag` 0)
    (set `self.GazeFlag` 0)))

(fn `DoStroke`
  (params (ObjectID :type Integer) (GazeAnimTime :type "Float (double-precision)"))
  (bind (_returnvalue_roll _returnvalue_pitch _returnvalue_yaw) (`KismetMathLibrary.BreakRotator` (`SceneComponent.K2_GetComponentRotation` (`Actor.RootComponent` (`self.CharactorRef`)))))
  (bind _value (`BlueprintMapLibrary.Map_Find` (`/Game/ARINBody/Blueprints/CH_ARINBody.ObjectArray` (`self.CharactorRef`)) ObjectID))
  (bind _returnvalue (- 180.0 (- (`KismetMathLibrary.Abs` (`self.TargetAngleX`)) 180.0)))
  (bind (_returnvalue_roll_2 _returnvalue_pitch_2 _returnvalue_yaw_2) (`KismetMathLibrary.BreakRotator` (`KismetMathLibrary.FindLookAtRotation` (+ (`SceneComponent.K2_GetComponentLocation` (`Actor.RootComponent` (`self.CharactorRef`))) (0.0 0.0 80.0)) _value)))
  (if (== (`self.State`) 0)
    (set `self.ObjectID` ObjectID)
    (set `self.TargetPosition` _value)
    ;[1 1 1] Set Anim Time
    (set `self.StrokeTime` GazeAnimTime)
    ;[1 1 1] SetAngle
    (bind _output_get (set `self.TargetAngleX` (- _returnvalue_yaw_2 _returnvalue_yaw)))
    (if (> (`KismetMathLibrary.Abs` (`self.TargetAngleX`)) 180.0)
      (if (> (`self.TargetAngleX`) 0.0)
        (set `self.TargetAngleX` (`KismetMathLibrary.FClamp` (* _returnvalue -1.0) -80.0 80.0))
        (else
          (set `self.TargetAngleX` (`KismetMathLibrary.FClamp` _returnvalue -80.0 80.0))))
      (else
        (set `self.TargetAngleX` (`KismetMathLibrary.FClamp` _output_get -80.0 80.0))))
    (set `self.TargetAngleY` (`KismetMathLibrary.FClamp` _returnvalue_pitch_2 -50.0 60.0))
    ;[1 1 1] Calculate Anim Time When Input Time is Negative
    (if (< (`self.StrokeTime`) 0.0)
      (set `self.StrokeTime` (`KismetMathLibrary.FClamp` (/ (`KismetMathLibrary.FMax` (`KismetMathLibrary.Abs` (- (`self.TargetAngleX`) (`self.CurAngleX`))) (`KismetMathLibrary.Abs` (- (`self.TargetAngleY`) (`self.CurAngleY`)))) 40.0) 0.5 2.0)))
    (if (<= (`|GetArrayItem` (`/Game/ARINBody/Blueprints/BP_ARINBody_AnimBlueprint.ControllerBlendAlphaArray` (`self.AnimBPref`)) (`KismetMathLibrary.Conv_ByteToInt` (enumliteral `/Game/ARINBody/Data/ControllerNameEnum` "NewEnumerator21"))) 0.0)
      ;[1 1 1] Calculate Gaze Angle when Gaze Upper Controller Attach
      (set `self.RelTargetAngleX` (`KismetMathLibrary.FClamp` (- (`self.TargetAngleX`) (`/Game/ARINBody/Blueprints/BP_ARINBody_AnimBlueprint.GazeUpperAngleX` (`self.AnimBPref`))) -80.0 80.0))
      (set `self.RelTargetAngleY` (`KismetMathLibrary.FClamp` (- (`self.TargetAngleY`) (`/Game/ARINBody/Blueprints/BP_ARINBody_AnimBlueprint.GazeUpperAngleY` (`self.AnimBPref`))) -50.0 60.0))
      ;[1 1 1] Calculate Anim Time When Input Time is Negative when Gaze Upper Controller Attach
      (`KismetArrayLibrary.Array_Set` (`/Game/ARINBody/Blueprints/BP_ARINBody_AnimBlueprint.AnimBlendAlphaArray` (`self.AnimBPref`)) (`self.ControllerNum`) 1.0)
      (if (< (`self.StrokeTime`) 0.0)
        (set `self.StrokeTime` (`KismetMathLibrary.FClamp` (/ (`KismetMathLibrary.FMax` (`KismetMathLibrary.Abs` (`self.RelTargetAngleX`)) (`KismetMathLibrary.Abs` (`self.RelTargetAngleY`))) 40.0) 0.5 2.0)))
      ;[1 1 1] Start Gaze Stroke and Set Flags
      (set `self.State` 3)
      (set `self.TurnFlag` 0)
      (set `self.GazeUpperFlag` 0)
      (set `self.GazeFlag` 0)
      (else
        ;[1 1 1] Start Gaze Stroke And Set Flags when GazeUpper Controller Detach
        (set `self.State` 1)
        (set `self.TurnFlag` 0)
        (set `self.GazeUpperFlag` 0)
        (set `self.GazeFlag` 0)))))

(fn `DoTurnReStroke`
  (params (Time :type "Float (double-precision)") (RotationAngle :type "Float (double-precision)"))
  (bind (_returnvalue_roll _returnvalue_pitch _returnvalue_yaw) (`KismetMathLibrary.BreakRotator` (`SceneComponent.K2_GetComponentRotation` (`Actor.RootComponent` (`self.CharactorRef`)))))
  (bind _returnvalue (- 180.0 (- (`KismetMathLibrary.Abs` (`self.TargetAngleX`)) 180.0)))
  (bind (_returnvalue_roll_2 _returnvalue_pitch_2 _returnvalue_yaw_2) (`KismetMathLibrary.BreakRotator` (`KismetMathLibrary.FindLookAtRotation` (+ (`SceneComponent.K2_GetComponentLocation` (`Actor.RootComponent` (`self.CharactorRef`))) (0.0 0.0 80.0)) (`self.TargetPosition`))))
  (if (== (`self.State`) 0)
    (if (<= (`|GetArrayItem` (`/Game/ARINBody/Blueprints/BP_ARINBody_AnimBlueprint.ControllerBlendAlphaArray` (`self.AnimBPref`)) (`self.ControllerNum`)) 0.0)
      ;[1 1 1] Set Anim Time
      (set `self.StrokeTime` Time)
      ;[1 1 1] Calculate X axis Angle
      (bind _output_get (set `self.TargetAngleX` (- _returnvalue_yaw_2 (+ _returnvalue_yaw RotationAngle))))
      (if (> (`KismetMathLibrary.Abs` (`self.TargetAngleX`)) 180.0)
        (if (> (`self.TargetAngleX`) 0.0)
          (set `self.TargetAngleX` (`KismetMathLibrary.FClamp` (* _returnvalue -1.0) -80.0 80.0))
          (else
            (set `self.TargetAngleX` (`KismetMathLibrary.FClamp` _returnvalue -80.0 80.0))))
        (else
          (set `self.TargetAngleX` (`KismetMathLibrary.FClamp` _output_get -80.0 80.0))))
      (if (<= (`|GetArrayItem` (`/Game/ARINBody/Blueprints/BP_ARINBody_AnimBlueprint.ControllerBlendAlphaArray` (`self.AnimBPref`)) (`KismetMathLibrary.Conv_ByteToInt` (enumliteral `/Game/ARINBody/Data/ControllerNameEnum` "NewEnumerator21"))) 0.0)
        ;[1 1 1] Set Start Point, Set Flags and Start Re Gaze Stroke when Upper Gaze Controller Attach
        (bind _output_get_2 (set `self.CurAngleY` (`self.TargetAngleY`)))
        (bind _output_get_3 (set `self.CurAngleX` (`self.TargetAngleX`)))
        (set `/Game/ARINBody/Blueprints/BP_ARINBody_AnimBlueprint.GazeAngleX` _output_get_3 (`self.AnimBPref`))
        (set `/Game/ARINBody/Blueprints/BP_ARINBody_AnimBlueprint.GazeAngleY` _output_get_2 (`self.AnimBPref`))
        (set `self.PrepTimer` 0.0)
        (set `self.State` 4)
        (set `self.TurnFlag` 0)
        (set `self.GazeUpperFlag` 0)
        (set `self.GazeFlag` 0)
        (else
          ;[1 1 1] Start Re Gaze Stroke when Upper Gaze Controller Detach
          (set `self.State` 1)
          (set `self.TurnFlag` 0)
          (set `self.GazeUpperFlag` 0)
          (set `self.GazeFlag` 0))))))

(fn `DoUpperGazeReStroke`
  (params (CurX :type "Float (double-precision)") (CurY :type "Float (double-precision)") (Time :type "Float (double-precision)"))
  (if (== (`self.State`) 0)
    (if (<= (`|GetArrayItem` (`/Game/ARINBody/Blueprints/BP_ARINBody_AnimBlueprint.ControllerBlendAlphaArray` (`self.AnimBPref`)) (`self.ControllerNum`)) 0.0)
      ;[1 1 1] Set Angles and Anim Time
      (set `self.StrokeTime` Time)
      (set `self.RelTargetAngleX` (`KismetMathLibrary.FClamp` (- (`self.TargetAngleX`) CurX) -80.0 80.0))
      (set `self.RelTargetAngleY` (`KismetMathLibrary.FClamp` (- (`self.TargetAngleY`) CurY) -50.0 60.0))
      ;[1 1 1] Set Relative Gaze Start Point
      (set `/Game/ARINBody/Blueprints/BP_ARINBody_AnimBlueprint.RelGazeAngleX` (`self.CurAngleX`) (`self.AnimBPref`))
      (set `/Game/ARINBody/Blueprints/BP_ARINBody_AnimBlueprint.RelGazeAngleY` (`self.CurAngleY`) (`self.AnimBPref`))
      ;[1 1 1] Start Stroke and Set Flags
      (`KismetArrayLibrary.Array_Set` (`/Game/ARINBody/Blueprints/BP_ARINBody_AnimBlueprint.AnimBlendAlphaArray` (`self.AnimBPref`)) (`self.ControllerNum`) 1.0)
      (set `self.State` 3)
      (set `self.TurnFlag` 0)
      (set `self.GazeUpperFlag` 0)
      (set `self.GazeFlag` 0))))

(fn `UserConstructionScript`)