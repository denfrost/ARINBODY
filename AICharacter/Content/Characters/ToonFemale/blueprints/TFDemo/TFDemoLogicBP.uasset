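; Logic Blueprint for the ToonFemale demo that animates facial morph targets on the player character's mesh.
; Data tables supply the Mixamo morph-name map and named preset weight sets; random functions can fill the weights or apply random morphs immediately.
; TriggerAnimation starts playback, and Tick calls PlayMorphTarget to ramp weights linearly up, then back down, by frame count rather than delta time.
; An init function stores references to the demo UI and Blueprint.
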(event `self.ReceiveTick`
  (params (DeltaSeconds :type "Float (single-precision)"))
  (`self.playMorphTarget`))

(fn `GenRandomAnim`
  (bind _facemorphtargets (`self.FaceMorphTargets`))
  (bind _keys (`BlueprintMapLibrary.Map_Keys` _facemorphtargets))
  (for _array_element _keys
    (`SkeletalMeshComponent.SetMorphTarget` (`Character.Mesh` (`GameplayStatics.GetPlayerCharacter` 0)) (`KismetStringLibrary.Conv_StringToName` (`BlueprintMapLibrary.Map_Find` _facemorphtargets _array_element)) (`KismetMathLibrary.RandomFloatInRange` 0.0 0.8) false)))

(fn `GetSelectedMorphVector`
  (params (ItemName :type String))
  (bind _returnvalue (`|GetDataTableRow` "/Game/Characters/ToonFemale/Data/PresetMixamoVector.PresetMixamoVector" (`KismetStringLibrary.Conv_StringToName` ItemName))
    (:`then`
      (set `self.FaceMorphMap` (`.BlendShape_6_922EB6984620C1CF3A7E948E60F8B281` (break `/Game/Characters/ToonFemale/Data/FaceMorphVector` _returnvalue))))))

(fn `InitalizeMorphMap`
  (bind _returnvalue (`|GetDataTableRow` "/Game/Characters/ToonFemale/Data/MixamoMorphMap.MixamoMorphMap" "Mixamo")
    (:`then`
      (set `self.FaceMorphTargets` (`.BlendShape_4_D729F2F945B5B8E8428C6CB451366845` (break `/Game/Characters/ToonFemale/Data/MorphTargetMap` _returnvalue))))))

(fn `InitializeTFDemoLogicBP`
  (params (TFDemoUI :type "/Game/Characters/ToonFemale/blueprints/TFDemo/TFDemoUI Object Reference") (TFDemoBP :type "/Game/Characters/ToonFemale/blueprints/TFDemo/TFDemoBP Object Reference"))
  (set `self.TFDemoUIRef` TFDemoUI)
  (set `self.TFDemoBPRef` TFDemoBP))

(fn `playMorphTarget`
  (bind _framenummax (`self.FrameNumMax`))
  (bind _facemorphmap (`self.FaceMorphMap`))
  (bind _returnvalue (`KismetMathLibrary.Conv_IntToDouble` _framenummax))
  (bind _mesh (`Character.Mesh` (`GameplayStatics.GetPlayerCharacter` 0)))
  (if (`self.IsPlayMorphAnimation`)
    (bind _result (`/Engine/EditorBlueprintResources/StandardMacros.IncrementInt` (`self.FrameNum`))
      (:`  `
        (if (<= _result (`KismetMathLibrary.FTrunc` (`KismetMathLibrary.Conv_IntToDouble` _framenummax)))
          (bind _keys (`BlueprintMapLibrary.Map_Keys` _facemorphmap))
          (for _array_element _keys
            (bind _returnvalue_2 (`KismetMathLibrary.Conv_IntToDouble` _result))
            (`SkeletalMeshComponent.SetMorphTarget` _mesh (`KismetStringLibrary.Conv_StringToName` _array_element) (* (/ (`BlueprintMapLibrary.Map_Find` _facemorphmap _array_element) (`KismetMathLibrary.Conv_IntToDouble` _framenummax)) _returnvalue_2) true))
          (else
            (bind _returnvalue_3 (- (* _returnvalue 2.0) _returnvalue_2))
            (if (>= _returnvalue_3 0.0)
              (bind _keys_2 (`BlueprintMapLibrary.Map_Keys` _facemorphmap))
              (for _array_element_2 _keys_2
                (`SkeletalMeshComponent.SetMorphTarget` _mesh (`KismetStringLibrary.Conv_StringToName` _array_element_2) (* (`BlueprintMapLibrary.Map_Find` _facemorphmap _array_element_2) (/ _returnvalue_3 _returnvalue)) true)))))))))

(fn `SetRandomMorphVector`
  (bind _keys (`BlueprintMapLibrary.Map_Keys` (`self.FaceMorphTargets`)))
  (for _array_element _keys
    (`BlueprintMapLibrary.Map_Add` (`self.FaceMorphMap`) _array_element (`KismetMathLibrary.RandomFloatInRange` 0.0 0.8)))
  (set `self.frameNum` 1)
  (set `self.IsPlayMorphAnimation` false))

(fn `TriggerAnimation`
  (set `self.IsPlayMorphAnimation` true)
  (set `self.frameNum` 1)
  (set `self.frameNumMax` 30))

(fn `UserConstructionScript`)